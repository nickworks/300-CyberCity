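; Audio visualizer actor showing one selected spectrum band as a pulsing, color-shifting sphere with a point light.
; Each Tick reads that band from an audio analysis object's spectrum and scales the sphere by its absolute value and an intensity setting.
; The normalized band value also drives color and emissive parameters on a dynamic material created at BeginPlay, plus the red channel of the light.
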(event `self.ReceiveBeginPlay`
  (`KismetArrayLibrary.Array_Set` (`self.SphereArray`) (`self.SpectrumSelection`) (`self.Sphere`))
  (bind _returnvalue (`PrimitiveComponent.CreateDynamicMaterialInstance` (`self.Sphere`) 0 "/Game/JordanJ_Content/Materials/AudioVFX/MID_DynamicBase.MID_DynamicBase" "None")))

(event `self.ReceiveTick`
  (params (DeltaSeconds :type "Float (single-precision)"))
  (bind _returnvalue (* (`self.Intensity`) 0.1))
  (bind _returnvalue_2 (`KismetMathLibrary.Abs` (`|GetArrayItem` (`self.Spectrum`) (`self.SpectrumSelection`))))
  (bind _returnvalue_3 (`KismetMathLibrary.NormalizeToRange` _returnvalue_2 0.0 35.0))
  (bind (_returnvalue_x _returnvalue_y _returnvalue_z) (`KismetMathLibrary.BreakVector` (`KismetMathLibrary.MakeVector` _returnvalue_2 _returnvalue_2 _returnvalue_2)))
  (bind _returnvalue_4 (* 4 _returnvalue_3))
  (set `self.Spectrum` (`/Game/JordanJ_Content/Blueprints/AudioAnalysis/BP_AudioPointWithAnalyzer.SpectrumAnalysis` (`self.Analysis`)))
  (`SceneComponent.SetRelativeScale3D` (`self.Sphere`) (`KismetMathLibrary.MakeVector` (* _returnvalue_x _returnvalue) (* _returnvalue_y _returnvalue) (* _returnvalue_z _returnvalue)))
  (bind _output_get (set `self.ColorParam` (make `LinearColor` _returnvalue_4 0.0 (`KismetMathLibrary.Abs` (- _returnvalue_3 1.0)) 1.0)))
  (bind _output_get_2 (set `self.ColorParam` (make `LinearColor` (`KismetMathLibrary.Exp` _returnvalue_4) 0.0 _returnvalue_3 1.0)))
  (`MaterialInstanceDynamic.SetVectorParameterValue` (stale `self.ReceiveBeginPlay` _returnvalue) "Color" (make `LinearColor` (break `LinearColor` _output_get) (`.G` (break `LinearColor` _output_get)) (`.B` (break `LinearColor` _output_get)) (`.A` (break `LinearColor` _output_get))))
  (`MaterialInstanceDynamic.SetVectorParameterValue` (stale `self.ReceiveBeginPlay` _returnvalue) "Emissive" (make `LinearColor` (break `LinearColor` _output_get_2) (`.G` (break `LinearColor` _output_get_2)) (`.B` (break `LinearColor` _output_get_2)) (`.A` (break `LinearColor` _output_get_2))))
  (`LightComponent.SetLightColor` (`self.PointLight`) (make `LinearColor` (* _returnvalue_3 0.5) 0.0 0.0 1.0) true))

(fn `UserConstructionScript`)