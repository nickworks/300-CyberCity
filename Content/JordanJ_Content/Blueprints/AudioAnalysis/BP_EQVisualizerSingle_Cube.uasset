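; Single-cube audio EQ visualizer that makes one shape glow in response to a selected band of the audio spectrum.
; BeginPlay stores the shape in an array at the band index and gives it a dynamic material instance.
; Each Tick reads that band from the Analysis spectrum, offsets and normalizes it, then applies an exponential curve to scale the base color.
; The result drives both the Color and Emissive material parameters.
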(event `self.ReceiveBeginPlay`
  (`KismetArrayLibrary.Array_Set` (`self.SphereArray`) (`self.SpectrumSelection`) (`self.Shape`))
  (bind _returnvalue (`PrimitiveComponent.CreateDynamicMaterialInstance` (`self.Shape`) 0 "/Game/JordanJ_Content/Materials/AudioVFX/MID_DynamicBase.MID_DynamicBase" "None")))

(event `self.ReceiveTick`
  (params (DeltaSeconds :type "Float (single-precision)"))
  (bind (_color_r _color_g _color_b) (break `LinearColor` (`self.Color`)))
  (bind _returnvalue (`KismetMathLibrary.Exp` (* 4 (`KismetMathLibrary.NormalizeToRange` (`KismetMathLibrary.Abs` (+ (`|GetArrayItem` (`self.Spectrum`) (`self.SpectrumSelection`)) 30.0)) 0.0 100.0))))
  (bind _returnvalue_2 (* _color_b _returnvalue))
  (bind _returnvalue_3 (* _color_r _returnvalue))
  (bind _returnvalue_4 (* _color_g _returnvalue))
  (set `self.Spectrum` (`/Game/JordanJ_Content/Blueprints/AudioAnalysis/BP_AudioPointWithAnalyzer.SpectrumAnalysis` (`self.Analysis`)))
  ;[1 1 1] Dynamic Material Manipulation (Refined)
  (bind _output_get (set `self.ColorParam` (make `LinearColor` _returnvalue_3 _returnvalue_4 _returnvalue_2 1.0)))
  (bind _output_get_2 (set `self.ColorParam` (make `LinearColor` _returnvalue_3 _returnvalue_4 _returnvalue_2 1.0)))
  (`MaterialInstanceDynamic.SetVectorParameterValue` (stale `self.ReceiveBeginPlay` _returnvalue) "Color" (make `LinearColor` (break `LinearColor` _output_get) (`.G` (break `LinearColor` _output_get)) (`.B` (break `LinearColor` _output_get)) (`.A` (break `LinearColor` _output_get))))
  (`MaterialInstanceDynamic.SetVectorParameterValue` (stale `self.ReceiveBeginPlay` _returnvalue) "Emissive" (make `LinearColor` (break `LinearColor` _output_get_2) (`.G` (break `LinearColor` _output_get_2)) (`.B` (break `LinearColor` _output_get_2)) (`.A` (break `LinearColor` _output_get_2)))))

(fn `UserConstructionScript`)