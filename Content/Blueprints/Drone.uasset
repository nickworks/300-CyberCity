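; Drone actor that homes in on the player, steering toward the last position where it had line of sight.
; Every tick it counts down a scan timer, periodically running a debug-drawn visibility trace to the player and updating Target only when nothing is hit.
; It then pushes Sphere1 with an acceleration-based force equal to the speed-clamped thrust vector toward Target minus current velocity, a simple seek steering behavior.
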(event `self.ReceiveTick`
  (params (DeltaSeconds :type "Float (single-precision)"))
  (`self.ScanForPlayer`)
  (`self.MoveTowardsTarget`))

(fn `MoveTowardsTarget`
  (`PrimitiveComponent.AddForce` (`self.Sphere1`) (- (`KismetMathLibrary.ClampVectorSize` (* (`KismetMathLibrary.Normal` (- (`self.Target`) (`self.K2_GetActorLocation`))) (`self.ThrustAmount`)) 0.0 (`self.MAX_SPEED`)) (`self.GetVelocity`)) "None" true))

(fn `ScanForPlayer`
  (if (> (`self.ScanTimer`) 0.0)
    (set `self.ScanTimer` (- (`self.ScanTimer`) (`GameplayStatics.GetWorldDeltaSeconds`)))
    (else
      (set `self.ScanTimer` 0.5)
      (bind (_outhit _returnvalue) (`KismetSystemLibrary.LineTraceSingle` :`Start` (`self.K2_GetActorLocation`) :`End` (`self.K2_GetActorLocation` (`GameplayStatics.GetPlayerCharacter` 0)) :`TraceChannel` "TraceTypeQuery1" :`DrawDebugType` "ForDuration"))
      (if (not _returnvalue)
        (set `self.Target` (`self.K2_GetActorLocation` (`GameplayStatics.GetPlayerCharacter` 0)))))))

(fn `UserConstructionScript`)