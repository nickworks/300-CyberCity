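; PickupGB is a collectible pickup that adds one to the player's GBTOTAL counter.
; On BeginPlay, a Spin timeline drives the Cube's yaw to animate it.
; When a CyborgPlayer overlaps the Cube, it increments the counter, plays a teleport sound cue at its location and destroys itself.
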(event `self.ReceiveBeginPlay`
  (bind (_direction _yaw) (`Timeline|Spin`)
    (:`Update`
      (`SceneComponent.K2_SetRelativeRotation` (`self.Cube`) (`KismetMathLibrary.MakeRotator` 0.0 0.0 _yaw) false true))))

(event `self.Cube.OnComponentBeginOverlap`
  (params (OverlappedComponent :type "PrimitiveComponent Object Reference") (OtherActor :type "Actor Object Reference") (OtherComp :type "PrimitiveComponent Object Reference") (OtherBodyIndex :type Integer) (bFromSweep :type Boolean) (SweepResult :type "HitResult Structure (by ref)"))
  (bind _ascyborg_player (cast `/Game/Blueprints/PlayerStuff/CyborgPlayer` OtherActor))
  (set `/Game/Blueprints/PlayerStuff/CyborgPlayer.GB TOTAL` (+ (`/Game/Blueprints/PlayerStuff/CyborgPlayer.GB TOTAL` _ascyborg_player) 1) _ascyborg_player)
  (`GameplayStatics.PlaySoundAtLocation` "/Engine/VREditor/Sounds/VR_teleport_Cue.VR_teleport_Cue" (`self.K2_GetActorLocation`) (struct) 1.0 1.0 0.0 null null null)
  (`self.K2_DestroyActor`))

(fn `UserConstructionScript`)