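; Enemy pawn base logic: tracks health, senses pawns through AI Perception, shoots projectiles at them and can explode.
; Perception updates cache the sensed pawn and its location, which feed the sight, shooting and distance-to-target helpers.
; Sight checks and shots run on delta-time countdown cooldowns; line-trace visibility code is left unconnected.
; Depleted health only switches the alert state; nothing here calls the helpers or Explode.
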(event `self.ReceiveAnyDamage`
  (params (Damage :type "Float (single-precision)") (DamageType :type "DamageType Object Reference") (InstigatedBy :type "Controller Object Reference") (DamageCauser :type "Actor Object Reference"))
  ;[1 1 1] Take damage
  (bind _output_get (set `self.Health` (- (`self.Health`) Damage)))
  (if (<= _output_get 0.0)
    (set `self.StateAlert` "NewEnumerator4")))

(event `self.AIPerception.OnPerceptionUpdated`
  (params (UpdatedActors :type "Array of Actor Object Reference (by ref)"))
  (`self.CheckForPerception`))

(fn `CheckForPerception`
  (bind _outactors (`AIPerceptionComponent.GetCurrentlyPerceivedActors` (`self.AIPerception`) null))
  (if (<= (`KismetArrayLibrary.Array_Length` _outactors) 0)
    (set `self.SensedPawn` null)
    (else
      (for _array_element _outactors
        (bind _aspawn (cast `Pawn` _array_element))
        (bind _output_get (set `self.SensedPawn` _aspawn))
        (set `self.SensedPawnLocation` (`self.K2_GetActorLocation` _output_get))))))

(fn `Explode`
  (`GameplayStatics.SpawnEmitterAtLocation` "/Game/Particles/Explosion.Explosion" (`self.K2_GetActorLocation`))
  (`self.K2_DestroyActor`))

(fn `IsAtTarget`
  (params (Threshold :type "Float (double-precision)" :default 200.0))
  (returns (IsAtTarget :type Boolean))
  (bind _threshold (`local.Threshold`))
  (return (<= (`KismetMathLibrary.VSizeSquared` (- (`self.SensedPawnLocation`) (`self.K2_GetActorLocation`))) (* _threshold _threshold))))

(fn `IsPlayerSeen`
  (params (CheckEvery :type "Float (double-precision)" :default 0.5))
  (returns (IsPlayerSeen :type Boolean) (LookedThisFrame :type Boolean))
  ;[1 1 1] Cooldown
  (if (> (`self.CooldownScan`) 0.0)
    (set `self.CooldownScan` (- (`self.CooldownScan`) (`GameplayStatics.GetWorldDeltaSeconds`)))
    (return false false)
    (else
      (set `self.CooldownScan` CheckEvery)
      ;[1 1 1] Check AIPerception whether or not the pawn is SEEN
      (`/Engine/EditorBlueprintResources/StandardMacros.IsValid` (`self.SensedPawn`)
        (:`Is Valid`
          (if (>= (`KismetArrayLibrary.Array_Find` (`AIPerceptionComponent.GetCurrentlyPerceivedActors` (`self.AIPerception`) "/Script/AIModule.AISense_Sight") (`self.SensedPawn`)) 0)
            (set `self.SensedPawnLocation` (`self.K2_GetActorLocation` (`self.SensedPawn`)))
            (return true true)
            (else
              (return false true))))
        (:`Is Not Valid`
          (return false true))))))

(fn `ShootAtPlayer`
  (params (`Projectile Type` :type "/Game/Blueprints/Weapons/Projectiles/Projectile Class Reference") (ShootOrigin :type "Vector Structure") (ShootCooldown :type "Float (double-precision)" :default 0.5))
  ;[1 1 1] Cooldown
  (if (>= (`self.CooldownShoot`) 0.0)
    (set `self.CooldownShoot` (- (`self.CooldownShoot`) (`GameplayStatics.GetWorldDeltaSeconds`)))
    (else
      (set `self.CooldownShoot` ShootCooldown)
      (`/Engine/EditorBlueprintResources/StandardMacros.IsValid` (`self.SensedPawn`)
        (:`Is Valid`
          (`|SpawnActorFromClass` (`local.Projectile Type`) (`KismetMathLibrary.MakeTransform` (`local.ShootOrigin`) (`KismetMathLibrary.FindLookAtRotation` (`local.ShootOrigin`) (`self.K2_GetActorLocation` (`self.SensedPawn`)))) "Undefined" "OverrideRootScale" null null))))))

(fn `UserConstructionScript`)