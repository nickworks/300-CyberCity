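; Flying drone enemy that investigates, pursues and shoots at sensed pawns, and explodes when dying.
; Tick runs an alert state machine: sight checks switch it between Aggro and Pursuing, waits return it to Idle, and Notify forces pursuit.
; Movement applies clamped velocity-steering forces to the capsule, while rotation interpolates toward the target or travel direction.
; Construction script sets custom depth stencil values marking the mesh as friendly or hostile.
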(event `self.ReceiveTick`
  (params (DeltaSeconds :type "Float (single-precision)"))
  (switch `/Game/Blueprints/AIPawnStates` (`self.StateAlert`)
    (:`NewEnumerator0`
      (`self.InvestigateSensedPawn`))
    (:`NewEnumerator1`
      (`self.TurnTowardsTarget`)
      (`self.WaitThenGoIdle` 2.0 :!label _label)
      (bind (_ispawnseen _lookedthisframe) (`self.IsSensedPawnInSight` 0.5 :!label _label_2))
      (if (and _ispawnseen _lookedthisframe)
        (`self.ChangeState` "NewEnumerator2")))
    (:`NewEnumerator7`
      (`self.TurnTowardsVelocity` 20.0)
      (bind _isattarget (`self.MoveTowardsTarget` 100.0))
      (if _isattarget
        (goto _label)
        (else
          (`self.WaitThenGoIdle` 4.0)
          (goto _label_2))))
    (:`NewEnumerator2`
      (`self.MoveTowardsTarget` 500.0)
      (`self.TurnTowardsTarget`)
      (`self.ShootAtPlayer` "/Game/Blueprints/Weapons/Projectiles/SlowProjectile.SlowProjectile_C" (+ (`self.K2_GetActorLocation`) (* (`KismetMathLibrary.Normal` (- (`self.SensedPawnLocation`) (`self.K2_GetActorLocation`))) 100.0)))
      (bind (_ispawnseen_2 _lookedthisframe_2) (`self.IsSensedPawnInSight` 0.5))
      (if (and (not _ispawnseen_2) _lookedthisframe_2)
        (`self.ChangeState` "NewEnumerator7")))
    (:`NewEnumerator4`
      (`self.Explode`))))

(event `self.Notify`
  (params (TriggeringPawn :type "Pawn Object Reference"))
  (`parent.Notify` TriggeringPawn)
  (`self.ChangeState` "NewEnumerator7"))

(fn `MoveTowardsTarget`
  (params (Threshold :type "Float (double-precision)"))
  (returns (IsAtTarget :type Boolean))
  (bind _isattarget (`self.IsAtTarget` Threshold))
  (if _isattarget
    (return true)
    (else
      ;[1 1 1] Movement (steering)
      (`PrimitiveComponent.AddForce` (`self.Capsule`) (- (`KismetMathLibrary.ClampVectorSize` (* (`KismetMathLibrary.Normal` (- (`self.SensedPawnLocation`) (`self.K2_GetActorLocation`))) (`self.ThrustAmount`)) 0.0 (`self.MAX_SPEED`)) (`self.GetVelocity`)) "None" true))))

(fn `TurnTowardsTarget`
  (`self.K2_SetActorRotation` (`KismetMathLibrary.RInterpTo` (`self.K2_GetActorRotation`) (`KismetMathLibrary.FindLookAtRotation` (`self.K2_GetActorLocation`) (`self.SensedPawnLocation`)) (`GameplayStatics.GetWorldDeltaSeconds`) 10.0)))

(fn `TurnTowardsVelocity`
  (params (SpeedThreshold :type "Float (double-precision)"))
  (bind _returnvalue (`self.GetVelocity`))
  (if (>= (`KismetMathLibrary.VSizeSquared` _returnvalue) (* SpeedThreshold SpeedThreshold))
    (`self.K2_SetActorRotation` (`KismetMathLibrary.RInterpTo` (`self.K2_GetActorRotation`) (`KismetMathLibrary.FindLookAtRotation` (`KismetMathLibrary.MakeVector` 0.0) _returnvalue) (`GameplayStatics.GetWorldDeltaSeconds`) 10.0))))

(fn `UpdateThreatSignature`
  (`PrimitiveComponent.SetCustomDepthStencilValue` (`self.Sphere`) (select `bool` (`self.IsFriendly`) :`false` 1 :`true` 2))
  (`PrimitiveComponent.SetCustomDepthStencilValue` (`self.Cone`) (select `bool` (`self.IsFriendly`) :`false` 1 :`true` 2)))

(fn `UserConstructionScript`
  (`self.UpdateThreatSignature`))