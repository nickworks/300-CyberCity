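; Missile launcher enemy that investigates sensed pawns and fires homing rockets at them.
; Tick runs an alert state machine: periodic raycast sight checks switch it between Investigating and Aggro, and Dying triggers Explode.
; While Aggro, Shoot spawns rockets from the Arrow on a slightly randomized cooldown, homing on the sensed pawn.
; UpdateThreatSignature marks friend or foe through custom depth stencil values on its meshes.
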(event `self.ReceiveTick`
  (params (DeltaSeconds :type "Float (single-precision)"))
  (switch `/Game/Blueprints/AIPawnStates` (`self.StateAlert`)
    (:`NewEnumerator0`
      (`self.InvestigateSensedPawn`))
    (:`NewEnumerator1`
      (bind (_ispawnseen _lookedthisframe) (`self.IsSensedPawnInSight` 1.0 true :!label _label))
      (if _lookedthisframe
        (`self.ChangeState` (select `bool` _ispawnseen :`false` "NewEnumerator1" :`true` "NewEnumerator2" :!type "/Game/Blueprints/AIPawnStates Enum"))))
    (:`NewEnumerator2`
      (`self.Shoot` 2.5)
      (goto _label))
    (:`NewEnumerator4`
      (`self.Explode`))))

(event `self.UpdateThreatSignature`
  (`PrimitiveComponent.SetCustomDepthStencilValue` (`self.Cube`) (select `bool` (`self.IsFriendly`) :`false` 1 :`true` 2))
  (`PrimitiveComponent.SetCustomDepthStencilValue` (`self.Sphere`) (select `bool` (`self.IsFriendly`) :`false` 1 :`true` 2))
  (`PrimitiveComponent.SetCustomDepthStencilValue` (`self.Cylinder1`) (select `bool` (`self.IsFriendly`) :`false` 1 :`true` 2)))

(fn `Shoot`
  (params (Delay :type "Float (double-precision)"))
  (bind (_returnvalue_location _returnvalue_rotation) (`KismetMathLibrary.BreakTransform` (`SceneComponent.K2_GetComponentToWorld` (`self.Arrow`))))
  (if (<= (`self.CooldownShoot`) 0.0)
    (set `self.CooldownShoot` (+ Delay (`KismetMathLibrary.RandomFloatInRange` -0.2 0.2)))
    (bind _returnvalue (`|SpawnActorFromClass` "/Game/Blueprints/Weapons/Projectiles/RocketProjectile.RocketProjectile_C" (`KismetMathLibrary.MakeTransform` _returnvalue_location _returnvalue_rotation) "Undefined" "OverrideRootScale" null null))
    (`/Game/Blueprints/Weapons/Projectiles/Projectile.SetHomingTarget` _returnvalue (`self.SensedPawn`))
    (else
      (set `self.CooldownShoot` (- (`self.CooldownShoot`) (`GameplayStatics.GetWorldDeltaSeconds`))))))

(fn `UserConstructionScript`)