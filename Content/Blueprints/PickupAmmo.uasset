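; Ammo pickup actor that grants the CyborgPlayer fixed amounts of five ammo types at once.
; A Spin timeline started on BeginPlay drives the Cube's yaw.
; When a CyborgPlayer overlaps the Cube, it calls PickupAmmo on GameMode_CyborgPlayer for each type, plays a sound at its location and destroys itself.
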(event `self.ReceiveBeginPlay`
  (bind (_direction _yaw) (`Timeline|Spin`)
    (:`Update`
      (`SceneComponent.K2_SetRelativeRotation` (`self.Cube`) (`KismetMathLibrary.MakeRotator` 0.0 0.0 _yaw) false true))))

(event `self.Cube.OnComponentBeginOverlap`
  (params (OverlappedComponent :type "PrimitiveComponent Object Reference") (OtherActor :type "Actor Object Reference") (OtherComp :type "PrimitiveComponent Object Reference") (OtherBodyIndex :type Integer) (bFromSweep :type Boolean) (SweepResult :type "HitResult Structure (by ref)"))
  (cast `/Game/Blueprints/PlayerStuff/CyborgPlayer` OtherActor)
  (bind _asgame_mode_cyborg_player (cast `/Game/Blueprints/PlayerStuff/GameMode_CyborgPlayer` (`GameplayStatics.GetGameMode`)))
  (`/Game/Blueprints/PlayerStuff/GameMode_CyborgPlayer.PickupAmmo` _asgame_mode_cyborg_player "NewEnumerator0" 10.0)
  (`/Game/Blueprints/PlayerStuff/GameMode_CyborgPlayer.PickupAmmo` _asgame_mode_cyborg_player "NewEnumerator1" 3.0)
  (`/Game/Blueprints/PlayerStuff/GameMode_CyborgPlayer.PickupAmmo` _asgame_mode_cyborg_player "NewEnumerator2" 20.0)
  (`/Game/Blueprints/PlayerStuff/GameMode_CyborgPlayer.PickupAmmo` _asgame_mode_cyborg_player "NewEnumerator3" 16.0)
  (`/Game/Blueprints/PlayerStuff/GameMode_CyborgPlayer.PickupAmmo` _asgame_mode_cyborg_player "NewEnumerator4" 8.0)
  (`GameplayStatics.PlaySoundAtLocation` "/Engine/VREditor/Sounds/VR_teleport_Cue.VR_teleport_Cue" (`self.K2_GetActorLocation`) (struct) 1.0 1.0 0.0 null null null)
  (`self.K2_DestroyActor`))

(fn `UserConstructionScript`)