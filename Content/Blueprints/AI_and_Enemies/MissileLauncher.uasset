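; AI missile launcher turret that fires homing rockets at its target and can be friendly or hostile, marked via custom depth stencil.
; Tick runs a state machine: idle, spinning search, pursuing, aggro, reloading and dying, with timed raycast sight checks driving transitions.
; Aggro fires bursts on a randomized cooldown, reusing Pursuing's smoothed yaw tracking between shots.
; Launch pitch interpolates with horizontal distance to the target.
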(event `self.ReceiveTick`
  (params (DeltaSeconds :type "Float (single-precision)"))
  (`parent.ReceiveTick` DeltaSeconds)
  (switch `/Game/Blueprints/AI_and_Enemies/AIPawnStates` (`self.CurrentState`)
    (:`NewEnumerator0`
      (`self.If Perceive Target Switch To` "NewEnumerator1"))
    (:`NewEnumerator1`
      (`self.Turn in Circles` 0.5)
      (`self.Wait Then Change To` 8.0)
      (bind (_ispawnseen _lookedthisframe) (`self.IsSensedPawnInSight` 0.5 true))
      (if _lookedthisframe
        (if _ispawnseen
          (`self.ChangeState` "NewEnumerator2"))))
    (:`NewEnumerator7`
      (`self.Turn Towards Target` :!label _label)
      (bind (_ispawnseen_2 _lookedthisframe_2) (`self.IsSensedPawnInSight` 1.0 true))
      (if _lookedthisframe_2
        (if _ispawnseen_2
          (`self.ChangeState` "NewEnumerator2")
          (else
            (`self.ChangeState` "NewEnumerator1")))))
    (:`NewEnumerator2`
      (bind _should_continue (`self.Shoot` 0.25))
      (if _should_continue
        (`self.Aim Pitch at Enemy` 1.0)
        (goto _label)))
    (:`NewEnumerator4`
      (`self.Explode`))
    (:`NewEnumerator9`
      (`self.Wait Then Change To` (`self.how long it takes to reload`) "NewEnumerator7")
      (set `self.how many shots taken` 0))))

(event `self.UpdateThreatSignature`
  (`PrimitiveComponent.SetCustomDepthStencilValue` (`self.Cube`) (select `bool` (`self.IsFriendly`) :`false` 1 :`true` 2))
  (`PrimitiveComponent.SetCustomDepthStencilValue` (`self.YawControl`) (select `bool` (`self.IsFriendly`) :`false` 1 :`true` 2))
  (`PrimitiveComponent.SetCustomDepthStencilValue` (`self.Cylinder1`) (select `bool` (`self.IsFriendly`) :`false` 1 :`true` 2)))

(fn `Aim Pitch at Enemy`
  (params (`Relative speed` :type "Float (double-precision)" :default 1.0))
  (bind _current_attack_target (`self.Current Attack Target`))
  (bind (_returnvalue_x _returnvalue_y) (`KismetMathLibrary.BreakVector` (- (`self.K2_GetActorLocation` _current_attack_target) (`SceneComponent.K2_GetComponentLocation` (`self.PitchControl`)))))
  (`/Engine/EditorBlueprintResources/StandardMacros.IsValid` _current_attack_target
    (:`Is Valid`
      (`SceneComponent.K2_SetRelativeRotation` (`self.PitchControl`) (`KismetMathLibrary.MakeRotator` (`KismetMathLibrary.Lerp` -150.0 -45.0 (/ (`KismetMathLibrary.VSize` (`KismetMathLibrary.MakeVector` _returnvalue_x _returnvalue_y)) 50000.0))) false false))))

(fn `Shoot`
  (params (Delay :type "Float (double-precision)"))
  (returns (`Should Continue` :type Boolean))
  (bind (_returnvalue_location _returnvalue_rotation) (`KismetMathLibrary.BreakTransform` (`SceneComponent.K2_GetComponentToWorld` (`self.Arrow`))))
  (if (< (`self.how many shots taken`) (`self.how many shots before reloading`))
    (if (<= (`self.CooldownShoot`) 0.0)
      (set `self.CooldownShoot` (+ Delay (`KismetMathLibrary.RandomFloatInRange` -0.2 0.2)))
      (bind _returnvalue (`|SpawnActorFromClass` "/Game/Blueprints/WeaponStuff/Projectiles/HomingRocket.HomingRocket_C" (`KismetMathLibrary.MakeTransform` _returnvalue_location _returnvalue_rotation) "Undefined" "OverrideRootScale" null null))
      (`/Engine/EditorBlueprintResources/StandardMacros.IncrementInt` (`self.how many shots taken`)
        (:`  `
          (`/Game/Blueprints/WeaponStuff/Projectiles/Projectile.SetHomingTarget` _returnvalue (`self.Current Attack Target`))
          (return false)))
      (else
        (set `self.CooldownShoot` (- (`self.CooldownShoot`) (`self.tick DT`)))
        (return true)))
    (else
      (`self.ChangeState` "NewEnumerator9")
      (return false))))

(fn `Turn in Circles`
  (params (`Relative speed` :type "Float (double-precision)" :default 1.0))
  (`SceneComponent.K2_SetWorldRotation` (`self.YawControl`) (`KismetMathLibrary.MakeRotator` 0.0 0.0 (+ (.yaw (`SceneComponent.K2_GetComponentRotation` (`self.YawControl`))) (* (`self.tick DT`) 360.0 `Relative speed`))) false false))

(fn `Turn Towards Target`
  (locals (`Angle Goal` :type "Float (double-precision)" :default 0.0))
  (bind _current_attack_target (`self.Current Attack Target`))
  (bind _yawcontrol (`self.YawControl`))
  (bind (_returnvalue_roll _returnvalue_pitch _returnvalue_yaw) (`KismetMathLibrary.BreakRotator` (`SceneComponent.K2_GetComponentRotation` (`self.YawControl`))))
  (bind (_returnvalue_roll_2 _returnvalue_pitch_2 _returnvalue_yaw_2) (`KismetMathLibrary.BreakRotator` (`KismetMathLibrary.FindLookAtRotation` (`SceneComponent.K2_GetComponentLocation` (`self.YawControl`)) (`self.K2_GetActorLocation` _current_attack_target))))
  (`/Engine/EditorBlueprintResources/StandardMacros.IsValid` _current_attack_target
    (:`Is Valid`
      (bind _output_get (set `local.Angle Goal` (+ _returnvalue_yaw_2 -90.0)))
      (bind _returnvalue (- _output_get _returnvalue_yaw))
      (if (> _returnvalue 180.0)
        (set `local.Angle Goal` (+ (`local.Angle Goal`) -360.0))
        (elif (< _returnvalue -180.0)
          (set `local.Angle Goal` (+ (`local.Angle Goal`) 360.0))))
      (`SceneComponent.K2_SetWorldRotation` _yawcontrol (`KismetMathLibrary.RLerp` (`SceneComponent.K2_GetComponentRotation` _yawcontrol) (`KismetMathLibrary.MakeRotator` 0.0 0.0 (`local.Angle Goal`)) 0.05) false false))))

(fn `UserConstructionScript`)