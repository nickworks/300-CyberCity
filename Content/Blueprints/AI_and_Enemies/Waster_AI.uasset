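; AI controller for the Waster enemy that chases CyborgPlayer targets using a simple Idle/Searching state machine run on Tick.
; Idle calls NewTarget, which reads the pawn's AIPerception only if AttackTarget is already valid, then switches to Searching when the target is valid.
; Searching moves to the target each tick and returns to Idle when it becomes invalid.
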(event `self.ReceiveBeginPlay`
  (`KismetSystemLibrary.PrintString` "Hello"))

(event `self.ReceiveTick`
  (params (DeltaSeconds :type "Float (single-precision)"))
  (switch `/Game/Blueprints/AI_and_Enemies/WasterStates` (`self.State`)
    (:`NewEnumerator0`
      (`self.New Target`)
      (`self.Idle->Search`))
    (:`NewEnumerator1`
      (`self.Pursue`))))

(fn `Change State`
  (params (NewParam :type "/Game/Blueprints/AI_and_Enemies/WasterStates Enum" :default "NewEnumerator0"))
  (set `self.State` NewParam))

(fn `Idle->Search`
  (`/Engine/EditorBlueprintResources/StandardMacros.IsValid` (`self.Attack Target`)
    (:`Is Valid`
      (`self.Change State` "NewEnumerator1"))))

(fn `New Target`
  (`/Engine/EditorBlueprintResources/StandardMacros.IsValid` (`self.Attack Target`)
    (:`Is Valid`
      (bind _aswaster (cast `/Game/Blueprints/AI_and_Enemies/Waster` (`self.K2_GetPawn`)))
      (for _array_element (`AIPerceptionComponent.GetCurrentlyPerceivedActors` (`/Game/Blueprints/AI_and_Enemies/Waster.AIPerception` _aswaster) null)
        (bind _ascyborg_player (cast `/Game/Blueprints/PlayerStuff/CyborgPlayer` _array_element))
        (set `self.Attack Target` _ascyborg_player)
        (break)))))

(fn `Pursue`
  (`/Engine/EditorBlueprintResources/StandardMacros.IsValid` (`self.Attack Target`)
    (:`Is Valid`
      (`self.MoveToActor` (`self.Attack Target`) -3.0 true true true null))
    (:`Is Not Valid`
      (`self.Change State` "NewEnumerator0"))))

(fn `UserConstructionScript`)