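; Drone spawner enemy that launches drones on a cooldown, within optional total and simultaneous limits.
; Tick runs a state switch: Idle watches for targets, Dying explodes, and active states share the spawn countdown.
; New drones get a random horizontal home offset and upward kick, join the spawner's network, then pursue its target or return.
; Destroyed drones leave the tracked list, freeing slots, and a custom event sets the tube's friend-or-foe stencil.
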(event `Droid Destroyed` :!signature `self.OnDestroyed`
  (params (DestroyedActor :type "Actor Object Reference"))
  (bind _asdrone_base_class (cast `/Game/Blueprints/AI_and_Enemies/Enemies/DroneBaseClass` DestroyedActor))
  (clear `self.OnDestroyed` _asdrone_base_class)
  (`KismetArrayLibrary.Array_RemoveItem` (`self.Drones`) _asdrone_base_class))

(event `self.ReceiveTick`
  (params (DeltaSeconds :type "Float (single-precision)"))
  (bind _max_droids_total (`self.max droids total`))
  (`parent.ReceiveTick` DeltaSeconds)
  (switch `/Game/Blueprints/AI_and_Enemies/AIPawnStates` (`self.CurrentState`)
    (:`NewEnumerator0`
      (`self.If Perceive Target Switch To` "NewEnumerator1"))
    (:`NewEnumerator5`
      (if (<= (`self.delay until next spawn`) 0.0) :!label _label
        (if (or (< (`self.how many droids have spawned`) _max_droids_total) (== _max_droids_total 0))
          (if (< (`KismetArrayLibrary.Array_Length` (`self.Drones`)) (`self.max number of drones at once`))
            (bind _returnvalue (`self.Spawn a Drone`))
            (add `self.OnDestroyed` _returnvalue (delegate `Droid Destroyed`))))
        (else
          ;[1 1 1] Count-down timer
          (set `self.delay until next spawn` (- (`self.delay until next spawn`) (`self.tick DT`))))))
    (:`NewEnumerator1`
      (goto _label))
    (:`NewEnumerator7`
      (goto _label))
    (:`NewEnumerator2`
      (goto _label))
    (:`NewEnumerator4`
      (`self.Explode`))))

(event `CustomEvent`
  (`PrimitiveComponent.SetCustomDepthStencilValue` (`self.tube`) (select `bool` (`self.IsFriendly`) :`false` 1 :`true` 2)))

(fn `Spawn a Drone`
  (returns (ReturnValue :type "/Game/Blueprints/AI_and_Enemies/Enemies/DroneBaseClass Object Reference"))
  (locals (`New Drone` :type "/Game/Blueprints/AI_and_Enemies/Enemies/DroneBaseClass Object Reference"))
  (bind (_returnvalue_x _returnvalue_y) (`KismetMathLibrary.BreakVector` (`KismetMathLibrary.RandomUnitVector`)))
  (bind _new_drone (`local.New Drone`))
  (bind _current_network (`self.current network`))
  (bind _new_drone_2 (`local.New Drone`))
  (bind _current_attack_target (`self.Current Attack Target`))
  (bind _returnvalue (`SceneComponent.K2_GetComponentLocation` (`self.SpawnLocationDirection`)))
  (set `self.delay until next spawn` (`self.spawn cooldown`))
  (bind _returnvalue_2 (`|SpawnActorFromClass` (`self.Drones to Spawn`) (`KismetMathLibrary.MakeTransform` _returnvalue) "Undefined" "OverrideRootScale" null null))
  (bind _asdrone_base_class (cast `/Game/Blueprints/AI_and_Enemies/Enemies/DroneBaseClass` _returnvalue_2))
  (bind _output_get (set `local.New Drone` _asdrone_base_class))
  (`KismetArrayLibrary.Array_Add` (`self.Drones`) _output_get)
  (`/Engine/EditorBlueprintResources/StandardMacros.IncrementInt` (`self.how many droids have spawned`)
    (:`  `
      (`/Game/Blueprints/AI_and_Enemies/Enemies/DroneBaseClass.Set position as HOME` _new_drone (+ _returnvalue (0.0 0.0 0.0) (* (`KismetMathLibrary.Normal` (`KismetMathLibrary.MakeVector` _returnvalue_x _returnvalue_y)) (`self.child home distance`))))
      (`PrimitiveComponent.AddForce` (`Character.CapsuleComponent` _new_drone) (* (`SceneComponent.GetUpVector` (`self.SpawnLocationDirection`)) (* (`KismetMathLibrary.RandomFloatInRange` 0.5 1.0) 100000.0)) "None" true)
      (`/Engine/EditorBlueprintResources/StandardMacros.IsValid` _current_network
        (:`Is Valid`
          (`/Game/Blueprints/NetworkedSystem.Add Pawn to Network` _current_network (`local.New Drone`)))
        (:`Is Not Valid`
          _))
      (`/Engine/EditorBlueprintResources/StandardMacros.IsValid` _current_attack_target
        (:`Is Valid`
          (set `/Game/Blueprints/AI_and_Enemies/AIPawn.Current Attack Target` _current_attack_target _new_drone_2)
          (set `/Game/Blueprints/AI_and_Enemies/Enemies/DroneBaseClass.Flight target` (`self.K2_GetActorLocation` _current_attack_target) _new_drone_2)
          (`self.ChangeState` _new_drone_2 "NewEnumerator7"))
        (:`Is Not Valid`
          (`self.ChangeState` _new_drone_2 "NewEnumerator6")))
      (return (`local.New Drone`)))))

(fn `UserConstructionScript`)