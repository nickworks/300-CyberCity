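; Laser tripwire trigger that alerts AI when a CyborgPlayer overlaps its cylinder while switched on.
; An overlap activates a trip sound and notifies networked systems and subscribed pawns, pruning invalid ones, plus optionally every AIPawn within a radius.
; The construction script sizes the beam and adds instanced end meshes spanning its travel.
; TurnOnOrOff drives the sine-wave movement timeline and custom depth stencil of the cylinder, which is hidden from the main pass.
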(event `self.ReceiveBeginPlay`
  ;[1 1 1] Make the cylinder invisible :)
  (`PrimitiveComponent.SetRenderInMainPass` (`self.Cylinder Trigger`) false)
  (`self.Turn On or Off` (`self.Is Turned On`)))

(event `self.Cylinder Trigger.OnComponentBeginOverlap`
  (params (OverlappedComponent :type "PrimitiveComponent Object Reference") (OtherActor :type "Actor Object Reference") (OtherComp :type "PrimitiveComponent Object Reference") (OtherBodyIndex :type Integer) (bFromSweep :type Boolean) (SweepResult :type "HitResult Structure (by ref)"))
  (if (`self.Is Turned On`)
    (bind _ascyborg_player (cast `/Game/Blueprints/PlayerStuff/CyborgPlayer` OtherActor))
    (`ActorComponent.SetActive` (`self.SoundTrip`) true false)
    (`self.Notify all Subscribers` _ascyborg_player)
    (if (`self.Also notify ALL AI within the radius`)
      (`self.Notify all Pawns in radius` _ascyborg_player))))

(fn `Notify all Pawns in radius`
  (params (TriggeringPawn :type "Pawn Object Reference"))
  (bind _returnvalue (* (`self.Notifitcation RADIUS in meters`) 100.0))
  (bind _outactors (`GameplayStatics.GetAllActorsOfClass` "/Game/Blueprints/AI_and_Enemies/AIPawn.AIPawn_C"))
  (for _array_element _outactors
    (if (<= (`KismetMathLibrary.VSizeSquared` (- (`self.K2_GetActorLocation`) (`self.K2_GetActorLocation` _array_element))) (* _returnvalue _returnvalue))
      (`/Game/Blueprints/AI_and_Enemies/AIPawn.Notify` _array_element TriggeringPawn))))

(fn `Notify all Subscribers`
  (params (TriggeringPawn :type "Pawn Object Reference"))
  (locals (`number removed` :type Integer) (`number notified` :type Integer))
  (bind _result (`BlueprintSetLibrary.Set_ToArray` (`self.Networked Systems to Notify`)))
  (for _array_element _result
    (`/Game/Blueprints/NetworkedSystem.Notify All Of Threat` _array_element (`local.TriggeringPawn`)))
  (bind (_arrayindex _arrayelement) (`/Engine/EditorBlueprintResources/StandardMacros.ReverseForEachLoop` (`self.Pawns to Notify`))
    (:`LoopBody`
      (`/Engine/EditorBlueprintResources/StandardMacros.IsValid` _arrayelement
        (:`Is Valid`
          (`/Game/Blueprints/AI_and_Enemies/AIPawn.Notify` _arrayelement TriggeringPawn)
          (`/Engine/EditorBlueprintResources/StandardMacros.IncrementInt` (`local.number notified`)))
        (:`Is Not Valid`
          (`KismetArrayLibrary.Array_Remove` (`self.Pawns to Notify`) _arrayindex)
          (`/Engine/EditorBlueprintResources/StandardMacros.IncrementInt` (`local.number removed`)))))))

(fn `Turn Off`
  (`self.Turn On or Off` false))

(fn `Turn On`
  (`self.Turn On or Off` true))

(fn `Turn On or Off`
  (params (`Should it be on now?` :type Boolean))
  (bind _cylinder_trigger (`self.Cylinder Trigger`))
  (bind _lasermovement (`self.LaserMovement`))
  (bind _output_get (set `self.Is Turned On` `Should it be on now?`))
  (if _output_get
    (`PrimitiveComponent.SetCustomDepthStencilValue` _cylinder_trigger 1)
    (if (> (`self.Move Length`) 0.0)
      (`TimelineComponent.SetPlayRate` _lasermovement (/ 1.0 (`self.Move Time`)))
      (`TimelineComponent.Play` _lasermovement))
    (else
      (`PrimitiveComponent.SetCustomDepthStencilValue` _cylinder_trigger 0)
      (`TimelineComponent.Stop` _lasermovement))))

(fn `UserConstructionScript`
  (bind _laser_length (`self.Laser Length`))
  (bind _instancedstaticmesh (`self.InstancedStaticMesh`))
  (bind _returnvalue (+ (`self.Move Length`) 0.1))
  (`self.Turn On or Off` (`self.Is Turned On`))
  (`SceneComponent.SetRelativeScale3D` (`self.Cylinder Trigger`) (`KismetMathLibrary.MakeVector` 0.1 0.1 _laser_length))
  (`InstancedStaticMeshComponent.AddInstance` _instancedstaticmesh (`KismetMathLibrary.MakeTransform` (`KismetMathLibrary.MakeVector` 0.0 0.0 (* _laser_length 50.0)) (struct) (`KismetMathLibrary.MakeVector` _returnvalue 0.1 0.1)))
  (`InstancedStaticMeshComponent.AddInstance` _instancedstaticmesh (`KismetMathLibrary.MakeTransform` (`KismetMathLibrary.MakeVector` 0.0 0.0 (* _laser_length -50.0)) (struct) (`KismetMathLibrary.MakeVector` _returnvalue 0.1 0.1))))