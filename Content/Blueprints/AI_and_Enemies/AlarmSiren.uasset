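; Alarm siren built on a state-driven parent class that starts switched off and turns on when notified, overriding Notify without calling the parent.
; TurnOn and TurnOff toggle the Spin timeline, two spotlights, Niagara effect and audio.
; The timeline rotates the Scene component and pulses glow on a dynamic danger material.
; Tick runs the parent logic and calls Explode in the Dying state; the perception check is left unconnected.
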(event `self.ReceiveBeginPlay`
  (bind _returnvalue (`PrimitiveComponent.CreateDynamicMaterialInstance` (`self.LIGHT`) 0 "/Game/ArtKits/Materials/GlowDanger.GlowDanger" "None"))
  (set `self.DangerMAT` _returnvalue)
  (`self.Turn Off`))

(event `self.ReceiveTick`
  (params (DeltaSeconds :type "Float (single-precision)"))
  (`parent.ReceiveTick` DeltaSeconds)
  (switch `/Game/Blueprints/AI_and_Enemies/AIPawnStates` (`self.CurrentState`)
    (:`NewEnumerator4`
      (`self.Explode`))))

(fn `Notify`
  (params (TriggeringPawn :type "Pawn Object Reference"))
  (`self.Turn On`))

(fn `Turn Off`
  (`TimelineComponent.Stop` (`self.Spin`))
  (`MaterialInstanceDynamic.SetScalarParameterValue` (`self.DangerMAT`) "GlowIntensity" 0.0)
  (`LightComponent.SetIntensity` (`self.SpotLight`) 0.0)
  (`LightComponent.SetIntensity` (`self.SpotLight1`) 0.0)
  (`ActorComponent.SetActive` (`self.Niagara`) false false)
  (`ActorComponent.SetActive` (`self.Audio`) false false))

(fn `Turn On`
  (`TimelineComponent.Play` (`self.Spin`))
  (`LightComponent.SetIntensity` (`self.SpotLight`) 20000.0)
  (`LightComponent.SetIntensity` (`self.SpotLight1`) 20000.0)
  (`ActorComponent.SetActive` (`self.Niagara`) true false)
  (`ActorComponent.SetActive` (`self.Audio`) true false))

(fn `UserConstructionScript`)