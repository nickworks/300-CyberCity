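; Holographic advertising billboard whose shape is built from a few size parameters for ad width, height and shrink, and base height and depth.
; The construction script scales and places a bottom base cube, a back cube above it, and an upright holo plane in front of the back, inset by the shrink value.
; A thin projector piece sits atop the base, aligned to the plane's X position and inset width.
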(fn `UserConstructionScript`
  (locals (`z position of ad` :type "Float (double-precision)"))
  (bind _base_height (`self.base-height`))
  (bind _ad_shrink (`self.ad-shrink`))
  (bind _returnvalue (* (`self.base-depth`) 0.5))
  (bind _relativelocation_x (`KismetMathLibrary.BreakVector` (`SceneComponent.RelativeLocation` (`self.Holoplane`))))
  (set `local.z position of ad` (+ (* (`self.ad-height`) 50.0) (* (`self.base-height`) 100.0)))
  (`SceneComponent.K2_SetRelativeTransform` (`self.Holoplane`) (`KismetMathLibrary.MakeTransform` (`KismetMathLibrary.MakeVector` (* (`self.base-depth`) 0.5 50.0) 0.0 (`local.z position of ad`)) (struct :`Yaw` -90.0 :`Roll` 90.0) (`KismetMathLibrary.MakeVector` (- (`self.ad-width`) _ad_shrink) (- (`self.ad-height`) _ad_shrink) 1.0)) false false)
  (`SceneComponent.K2_SetRelativeTransform` (`self.Cube-Back`) (`KismetMathLibrary.MakeTransform` (`KismetMathLibrary.MakeVector` (* _returnvalue -50.0) 0.0 (`local.z position of ad`)) (struct) (`KismetMathLibrary.MakeVector` _returnvalue (`self.ad-width`) (`self.ad-height`))) false false)
  (`SceneComponent.K2_SetRelativeTransform` (`self.Cube-Bottom`) (`KismetMathLibrary.MakeTransform` (`KismetMathLibrary.MakeVector` 0.0 0.0 (* _base_height 50.0)) (struct) (`KismetMathLibrary.MakeVector` (`self.base-depth`) (`self.ad-width`) _base_height)) false false)
  (`SceneComponent.K2_SetRelativeTransform` (`self.Cube-ProjectoryBit`) (`KismetMathLibrary.MakeTransform` (`KismetMathLibrary.MakeVector` _relativelocation_x 0.0 (* (`self.base-height`) 100.0)) (struct) (`KismetMathLibrary.MakeVector` (- (* (`self.base-depth`) 0.5) 0.04) (- (`self.ad-width`) (`self.ad-shrink`)) 0.3)) false false))