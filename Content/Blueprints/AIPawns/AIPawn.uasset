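; Base AI pawn with health, a friendly/hostile allegiance and helper functions for sensing, investigating and shooting an attack target.
; AIPerception updates or Notify calls pick opposing pawns or the player as targets; sight checks use perception or a raycast.
; A state enum with Tick-delta cooldowns paces behavior, though no per-state update runs here.
; Allegiance sets custom depth stencil values on static meshes.
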(event `self.ReceiveAnyDamage`
  (params (Damage :type "Float (single-precision)") (DamageType :type "DamageType Object Reference") (InstigatedBy :type "Controller Object Reference") (DamageCauser :type "Actor Object Reference"))
  ;[1 1 1] Take damage
  (bind _output_get (set `self.Health` (- (`self.Health`) Damage)))
  (if (<= _output_get 0.0)
    (`self.ChangeState` "NewEnumerator4")))

(event `self.AIPerception.OnPerceptionUpdated`
  (params (UpdatedActors :type "Array of Actor Object Reference (by ref)"))
  (if (`|EnumInequality` (`self.CurrentState`) "NewEnumerator8")
    (`self.CheckForPerception`)))

(event `self.ReceiveTick`
  (params (DeltaSeconds :type "Float (single-precision)"))
  (set `self.tick DT` DeltaSeconds))

(event `self.ReceiveBeginPlay`
  (`self.UpdateThreatSignature`))

(fn `Awake`
  (if (`|EnumEquality` (`self.CurrentState`) "NewEnumerator8")
    (`self.ChangeState` "NewEnumerator0")))

(fn `ChangeFriendly`
  (params (IsFriendly :type Boolean))
  (set `self.IsFriendly` IsFriendly)
  (`self.UpdateThreatSignature`))

(fn `ChangeState`
  (params (state :type "/Game/Blueprints/AIPawns/AIPawnStates Enum" :default "NewEnumerator0"))
  (`self.ResetAllTimers`)
  (bind _output_get (set `self.CurrentState` state))
  (switch `/Game/Blueprints/AIPawns/AIPawnStates` _output_get
    (:`NewEnumerator0`
      (set `self.Current Attack Target` null))))

(fn `CheckForPerception`
  (bind _outactors (`AIPerceptionComponent.GetCurrentlyPerceivedActors` (`self.AIPerception`) null))
  (if (not (<= (`KismetArrayLibrary.Array_Length` _outactors) 0))
    (for _array_element _outactors
      (if (not (`self.IsFriendly`))
        ;[1 1 1] Not friendly: scan for a player...
        (bind _ascyborg_player (cast `/Game/Blueprints/PlayerStuff/CyborgPlayer` _array_element)
          (:`then`
            (set `self.Current Attack Target` _ascyborg_player)
            (set `self.SensedPawnLocation` (`self.K2_GetActorLocation` (`self.Current Attack Target`)) :!label _label)
            (break))
          (:`CastFailed`
            ;[1 1 1] Friendly: scan for AIPawns
            (bind _asaipawn (cast `/Game/Blueprints/AIPawns/AIPawn` _array_element :!label _label_2))
            (if (!= (`/Game/Blueprints/AIPawns/AIPawn.IsFriendly` _asaipawn) (`self.IsFriendly`))
              (set `self.Current Attack Target` _asaipawn)
              (goto _label))))
        (else
          (goto _label_2))))))

(fn `Explode`
  (`GameplayStatics.SpawnEmitterAtLocation` "/Game/ArtKits/Particles/Explosion.Explosion" (`self.K2_GetActorLocation`))
  (`self.K2_DestroyActor`))

(fn `InvestigateSensedPawn`
  (`/Engine/EditorBlueprintResources/StandardMacros.IsValid` (`self.Current Attack Target`)
    (:`Is Valid`
      (`self.ChangeState` "NewEnumerator1"))))

(fn `IsAtTarget`
  (params (Threshold :type "Float (double-precision)" :default 200.0))
  (returns (IsAtTarget :type Boolean))
  (bind _threshold (`local.Threshold`))
  (return (<= (`KismetMathLibrary.VSizeSquared` (- (`self.SensedPawnLocation`) (`self.K2_GetActorLocation`))) (* _threshold _threshold))))

(fn `IsSensedPawnInSight`
  (params (CheckEvery :type "Float (double-precision)" :default 0.5) (`Do a Raycast (instead of using Perception)` :type Boolean))
  (returns (IsPawnSeen :type Boolean) (LookedThisFrame :type Boolean))
  ;[1 1 1] Cooldown
  (if (> (`self.CooldownPerception`) 0.0)
    (set `self.CooldownPerception` (- (`self.CooldownPerception`) (`self.tick DT`)))
    (return false false)
    (else
      (set `self.CooldownPerception` CheckEvery)
      (`/Engine/EditorBlueprintResources/StandardMacros.IsValid` (`self.Current Attack Target`)
        (:`Is Valid`
          (if `Do a Raycast (instead of using Perception)`
            ;[1 1 1] Raycasting
            (bind (_outhit _returnvalue) (`KismetSystemLibrary.LineTraceSingle` :`Start` (`self.K2_GetActorLocation`) :`End` (`self.K2_GetActorLocation` (`self.Current Attack Target`)) :`TraceChannel` "TraceTypeQuery1" :`DrawTime` 0.5))
            (if (and (not _returnvalue) (<= (`.Distance` (`GameplayStatics.BreakHitResult` _outhit)) (`self.MaxVisibilityDistance`)))
              (set `self.SensedPawnLocation` (`self.K2_GetActorLocation` (`self.Current Attack Target`)))
              (return true true)
              (else
                (return false true)))
            (else
              ;[1 1 1] Check AIPerception whether or not the pawn is SEEN
              (if (>= (`KismetArrayLibrary.Array_Find` (`AIPerceptionComponent.GetCurrentlyPerceivedActors` (`self.AIPerception`) "/Script/AIModule.AISense_Sight") (`self.Current Attack Target`)) 0)
                (set `self.SensedPawnLocation` (`self.K2_GetActorLocation` (`self.Current Attack Target`)))
                (return true true)
                (else
                  (return false true))))))
        (:`Is Not Valid`
          (return false true))))))

(fn `Notify`
  (params (TriggeringPawn :type "Pawn Object Reference"))
  (bind _triggeringpawn (`local.TriggeringPawn`))
  (`self.Awake`)
  (bind _asaipawn (cast `/Game/Blueprints/AIPawns/AIPawn` TriggeringPawn)
    (:`then`
      ;[1 1 1] Trigger is an AI
      (if (!= (`/Game/Blueprints/AIPawns/AIPawn.IsFriendly` _asaipawn) (`self.IsFriendly`))
        (`/Engine/EditorBlueprintResources/StandardMacros.IsValid` (`self.Current Attack Target`) :!label _label ; If I don't already have a target...
          (:`Is Not Valid`
            ;[1 1 1] Set this as a new target for me
            (set `self.Current Attack Target` _triggeringpawn)
            (set `self.SensedPawnLocation` (`self.K2_GetActorLocation` _triggeringpawn))))))
    (:`CastFailed`
      ;[1 1 1] Trigger is a Player
      (if (`self.IsFriendly`)
        (`KismetSystemLibrary.PrintString` "I'm too friendly to attack the player")
        (else
          (goto _label))))))

(fn `ResetAllTimers`
  (set `self.CooldownStateChange` 0.0)
  (set `self.CooldownPerception` 0.0))

(fn `Shoot at Attack Target`
  (params (`Projectile Type` :type "/Game/Blueprints/Weapons/Projectiles/Projectile Class Reference") (ShootOrigin :type "Vector Structure") (ShootCooldown :type "Float (double-precision)" :default 0.5) (`Wants to Shoot` :type Boolean))
  (bind _capsulecomponent (`self.CapsuleComponent`))
  (if (>= (`self.CooldownShoot`) 0.0)
    (set `self.CooldownShoot` (- (`self.CooldownShoot`) (`self.tick DT`)))
    (elif `Wants to Shoot`
      (`/Engine/EditorBlueprintResources/StandardMacros.IsValid` (`self.Current Attack Target`)
        (:`Is Valid`
          (set `self.CooldownShoot` ShootCooldown)
          (`|SpawnActorFromClass` (`local.Projectile Type`) (`KismetMathLibrary.MakeTransform` (`local.ShootOrigin`) (`KismetMathLibrary.MakeRotationFromAxes` (`SceneComponent.GetForwardVector` _capsulecomponent) (`SceneComponent.GetRightVector` _capsulecomponent) (0.0 0.0 1.0))) "Undefined" "OverrideRootScale" null null))))))

(fn `UpdateThreatSignature`
  (bind _returnvalue (`self.K2_GetComponentsByClass` "/Script/Engine.StaticMeshComponent"))
  (`KismetSystemLibrary.PrintString` (`KismetStringLibrary.Conv_IntToString` (`KismetArrayLibrary.Array_Length` _returnvalue)))
  (for _array_element _returnvalue
    (`PrimitiveComponent.SetRenderCustomDepth` _array_element true)
    (`PrimitiveComponent.SetCustomDepthStencilValue` _array_element (select `bool` (`self.IsFriendly`) :`false` 1 :`true` 2))))

(fn `UserConstructionScript`)

(fn `Wait Then Change To`
  (params (Delay :type "Float (double-precision)") (state :type "/Game/Blueprints/AIPawns/AIPawnStates Enum" :default "NewEnumerator0"))
  (bind _output_get (set `self.CooldownStateChange` (+ (`self.CooldownStateChange`) (`self.tick DT`))))
  (if (>= _output_get Delay)
    (`self.ChangeState` state)))