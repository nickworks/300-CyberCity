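; D7WallLampStatic is a wall lamp Blueprint with a spotlight and a bulb mesh, configured through variables for light color, attenuation and intensity.
; The construction script applies those variables to the SpotLight.
; It also creates a dynamic material instance on the LightBulb and sets its Color and Emissive parameters to the light color, so bulb and light match.
; The event graph has no runtime logic.
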(event `self.ReceiveBeginPlay`)

(fn `UserConstructionScript`
  (bind _spotlight (`self.SpotLight`))
  (bind _lightcolor (`self.LightColor`))
  (`LightComponent.SetLightColor` _spotlight _lightcolor false)
  (`LocalLightComponent.SetAttenuationRadius` (`self.SpotLight`) (`self.LightAttentuation`))
  (`LightComponent.SetIntensity` _spotlight (`self.LightIntensity`))
  (bind _returnvalue (`PrimitiveComponent.CreateDynamicMaterialInstance` (`self.LightBulb`) 0 "/Game/Blueprints/JordanJ_Content/Materials/AudioVFX/MID_DynamicBase.MID_DynamicBase" "None"))
  (`MaterialInstanceDynamic.SetVectorParameterValue` _returnvalue "Color" _lightcolor)
  (`MaterialInstanceDynamic.SetVectorParameterValue` _returnvalue "Emissive" _lightcolor))