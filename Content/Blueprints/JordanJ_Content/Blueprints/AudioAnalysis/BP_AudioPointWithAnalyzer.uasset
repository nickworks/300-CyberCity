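; BP_AudioPointWithAnalyzer is a sound-emitting actor that plays a music track and analyzes its frequency spectrum as it plays.
; On BeginPlay it assigns Music to its audio component and plays it, replaying when finished if Loop is set.
; Each playback-percent update converts progress into a time position and runs CalculateFrequencySpectrum over a configurable window and width, storing the result in SpectrumAnalysis.
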(event `self.Audio.OnAudioFinished`
  ;[1 1 1] Set Music, Play, and Loop on finish
  (if (`self.Loop?`)
    (`AudioComponent.Play` (`self.Audio`) 0.0 :!label _label)))

(event `self.ReceiveBeginPlay`
  ;[1 1 1] Set Music, Play, and Loop on finish
  (`AudioComponent.SetSound` (`self.Audio`) (`self.Music`))
  (goto _label))

(event `self.Audio.OnAudioPlaybackPercent`
  (params (PlayingSoundWave :type "SoundWave Object Reference") (PlaybackPercent :type "Float (single-precision)"))
  (bind _music (`self.Music`))
  ;[1 1 1] Audio Analysis
  (bind _outspectrum (`SoundVisualizationStatics.CalculateFrequencySpectrum` _music 0 (* PlaybackPercent (`SoundBase.Duration` _music)) (`self.SpectrumWindow`) (`self.SpectrumWidth`)))
  (set `self.SpectrumAnalysis` _outspectrum))

(event `self.ReceiveTick`
  (params (DeltaSeconds :type "Float (single-precision)")))

(fn `UserConstructionScript`)