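; Audio spectrum visualizer actor that stretches and lights a row of ten mesh components in response to a soundtrack.
; BeginPlay gathers the components into an array and starts the soundtrack.
; Each Tick maps Analyzer spectrum bands by index to each component's Z scale, weighted by Intensity, and exponentially brightens the base Color for its Color and Emissive parameters.
; A new dynamic material instance is created for every component each frame.
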(event `self.ReceiveBeginPlay`
  (bind _spherearray (`self.SphereArray`))
  (`KismetArrayLibrary.Array_Set` _spherearray 0 (`self.Sphere`) true)
  (`KismetArrayLibrary.Array_Set` _spherearray 1 (`self.Sphere1`) true)
  (`KismetArrayLibrary.Array_Set` _spherearray 2 (`self.Sphere2`) true)
  (`KismetArrayLibrary.Array_Set` _spherearray 3 (`self.Sphere3`) true)
  (`KismetArrayLibrary.Array_Set` _spherearray 4 (`self.Sphere4`) true)
  (`KismetArrayLibrary.Array_Set` _spherearray 5 (`self.Sphere5`) true)
  (`KismetArrayLibrary.Array_Set` _spherearray 6 (`self.Sphere6`) true)
  (`KismetArrayLibrary.Array_Set` _spherearray 7 (`self.Sphere7`) true)
  (`KismetArrayLibrary.Array_Set` _spherearray 8 (`self.Sphere8`) true)
  (`KismetArrayLibrary.Array_Set` _spherearray 9 (`self.Sphere9`) true)
  (`AudioComponent.Play` (`self.Soundtrack`) 0.1))

(event `self.ReceiveTick`
  (params (DeltaSeconds :type "Float (single-precision)"))
  (bind (_color_r _color_g _color_b) (break `LinearColor` (`self.Color`)))
  (for (_array_element _array_index) (`self.SphereArray`)
    (bind _returnvalue (`PrimitiveComponent.CreateDynamicMaterialInstance` _array_element 0 "/Game/Blueprints/JordanJ_Content/Materials/AudioVFX/MID_DynamicBase.MID_DynamicBase" "None"))
    (bind _returnvalue_2 (`KismetMathLibrary.Abs` (`|GetArrayItem` (`/Game/Blueprints/JordanJ_Content/Blueprints/AudioAnalysis/BP_AudioPointWithAnalyzer.SpectrumAnalysis` (`self.Analyzer`)) _array_index)))
    (bind (_returnvalue_x _returnvalue_y _returnvalue_z) (`KismetMathLibrary.BreakVector` (`KismetMathLibrary.MakeVector` _returnvalue_2 _returnvalue_2 _returnvalue_2)))
    (`SceneComponent.SetRelativeScale3D` _array_element (`KismetMathLibrary.MakeVector` 1.0 1.0 (* (* _returnvalue_z (`self.Intensity`)) 0.05)))
    (bind _returnvalue_3 (`KismetMathLibrary.Exp` (* 4 (`KismetMathLibrary.NormalizeToRange` _returnvalue_2 0.0 100.0))))
    (bind _returnvalue_4 (* _color_r _returnvalue_3))
    (bind _returnvalue_5 (* _color_g _returnvalue_3))
    (bind _returnvalue_6 (* _color_b _returnvalue_3))
    ;[1 1 1] Dynamic Material Manipulation (Refined)
    (bind _output_get (set `self.ColorParam` (make `LinearColor` _returnvalue_4 _returnvalue_5 _returnvalue_6 1.0)))
    (bind _output_get_2 (set `self.ColorParam` (make `LinearColor` _returnvalue_4 _returnvalue_5 _returnvalue_6 1.0)))
    (`MaterialInstanceDynamic.SetVectorParameterValue` _returnvalue "Color" (make `LinearColor` (break `LinearColor` _output_get) (`.G` (break `LinearColor` _output_get)) (`.B` (break `LinearColor` _output_get)) (`.A` (break `LinearColor` _output_get))))
    (`MaterialInstanceDynamic.SetVectorParameterValue` _returnvalue "Emissive" (make `LinearColor` (break `LinearColor` _output_get_2) (`.G` (break `LinearColor` _output_get_2)) (`.B` (break `LinearColor` _output_get_2)) (`.A` (break `LinearColor` _output_get_2))))))

(fn `UserConstructionScript`)