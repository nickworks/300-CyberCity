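; Audio visualizer actor that makes one sphere and its point light react to a single selected band of an audio spectrum.
; BeginPlay creates the sphere's dynamic material instance.
; Each Tick reads the spectrum from the Analysis reference, scales the sphere by the offset band level and Intensity, then reruns the shared color update.
; That update boosts the base color exponentially with the level, driving material Color, Emissive and normalized light color.
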(event `self.ReceiveBeginPlay`
  (bind (_color_r _color_g _color_b) (break `LinearColor` (`self.Color`)))
  (bind _spectrumselection (`self.SpectrumSelection`))
  (bind _light_intensity (`self.Light Intensity`))
  (bind _returnvalue (`KismetMathLibrary.Exp` (* 4 (`KismetMathLibrary.NormalizeToRange` (`KismetMathLibrary.Abs` (+ (`|GetArrayItem` (`self.Spectrum`) _spectrumselection) 30.0)) 0.0 100.0))))
  (bind _returnvalue_2 (* _color_b _returnvalue))
  (bind _returnvalue_3 (* _color_r _returnvalue))
  (bind _returnvalue_4 (* _color_g _returnvalue))
  (`KismetArrayLibrary.Array_Set` (`self.SphereArray`) _spectrumselection (`self.Sphere`))
  ;[1 1 1] Dynamic Material Manipulation (Refined)
  (bind _returnvalue_5 (`PrimitiveComponent.CreateDynamicMaterialInstance` (`self.Sphere`) 0 "/Game/Blueprints/JordanJ_Content/Materials/AudioVFX/MID_DynamicBase.MID_DynamicBase" "None"))
  (bind _output_get (set `self.ColorParam` (make `LinearColor` _returnvalue_3 _returnvalue_4 _returnvalue_2 1.0) :!label _label))
  (bind _output_get_2 (set `self.ColorParam` (make `LinearColor` _returnvalue_3 _returnvalue_4 _returnvalue_2 1.0)))
  (`MaterialInstanceDynamic.SetVectorParameterValue` _returnvalue_5 "Color" (make `LinearColor` (break `LinearColor` _output_get) (`.G` (break `LinearColor` _output_get)) (`.B` (break `LinearColor` _output_get)) (`.A` (break `LinearColor` _output_get))))
  (`MaterialInstanceDynamic.SetVectorParameterValue` _returnvalue_5 "Emissive" (make `LinearColor` (break `LinearColor` _output_get_2) (`.G` (break `LinearColor` _output_get_2)) (`.B` (break `LinearColor` _output_get_2)) (`.A` (break `LinearColor` _output_get_2))))
  ;[1 1 1] Light Manipulation
  (`LightComponent.SetLightColor` (`self.PointLight`) (make `LinearColor` (* (`KismetMathLibrary.NormalizeToRange` _returnvalue_3 0.0 40.0) _light_intensity) (* (`KismetMathLibrary.NormalizeToRange` _returnvalue_4 0.0 40.0) _light_intensity) (* (`KismetMathLibrary.NormalizeToRange` _returnvalue_2 0.0 40.0) _light_intensity) 1.0) true))

(event `self.ReceiveTick`
  (params (DeltaSeconds :type "Float (single-precision)"))
  (bind _returnvalue (* (`self.Intensity`) 0.05))
  (bind _returnvalue_2 (`KismetMathLibrary.Abs` (+ (`|GetArrayItem` (`self.Spectrum`) (`self.SpectrumSelection`)) 30.0)))
  (bind (_returnvalue_x _returnvalue_y _returnvalue_z) (`KismetMathLibrary.BreakVector` (`KismetMathLibrary.MakeVector` _returnvalue_2 _returnvalue_2 _returnvalue_2)))
  ;[1 1 1] Analyzer Blueprint Call
  (set `self.Spectrum` (`/Game/Blueprints/JordanJ_Content/Blueprints/AudioAnalysis/BP_AudioPointWithAnalyzer.SpectrumAnalysis` (`self.Analysis`)))
  ;[1 1 1] Vector Manipulation
  (`SceneComponent.SetRelativeScale3D` (`self.Sphere`) (`KismetMathLibrary.MakeVector` (* _returnvalue_x _returnvalue) (* _returnvalue_y _returnvalue) (* _returnvalue_z _returnvalue)))
  (goto _label))

(fn `UserConstructionScript`)