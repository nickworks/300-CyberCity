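; A networked system Blueprint that links a set of pawns so threat alerts can be broadcast to all of them.
; Pawns are added to or removed from the set, and receive a reference to the system when added and again on BeginPlay.
; NotifyAllOfThreat relays a threat to each valid pawn, then rebuilds the set from those pawns to prune invalid references.
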(event `self.ReceiveBeginPlay`
  (`self.Ping All Connected`))

(fn `Add Pawn to Network`
  (params (Pawn :type "/Game/Blueprints/AI_and_Enemies/AIPawn Object Reference (by ref)"))
  (`BlueprintSetLibrary.Set_Add` (`self.Connected Pawns`) Pawn)
  (`/Game/Blueprints/AI_and_Enemies/AIPawn.Notify of Network Connection` Pawn self))

(fn `Notify All Of Threat`
  (params (Threat :type "Pawn Object Reference"))
  (locals (`Number notified` :type Integer) (`Number removed` :type Integer) (`Pawns kept` :type "Array of /Game/Blueprints/AI_and_Enemies/AIPawn Object Reference"))
  (bind _connected_pawns (`self.Connected Pawns`))
  (bind _result (`BlueprintSetLibrary.Set_ToArray` (`self.Connected Pawns`)))
  (for _array_element _result
    (`/Engine/EditorBlueprintResources/StandardMacros.IsValid` _array_element
      (:`Is Valid`
        (`/Game/Blueprints/AI_and_Enemies/AIPawn.Notify of Possible Threat` _array_element (`local.Threat`))
        (`/Engine/EditorBlueprintResources/StandardMacros.IncrementInt` (`local.Number notified`)
          (:`  `
            (`KismetArrayLibrary.Array_Add` (`local.Pawns kept`) _array_element))))
      (:`Is Not Valid`
        (`/Engine/EditorBlueprintResources/StandardMacros.IncrementInt` (`local.number removed`)))))
  (`BlueprintSetLibrary.Set_Clear` _connected_pawns)
  (`BlueprintSetLibrary.Set_AddItems` _connected_pawns (`local.Pawns kept`)))

(fn `Ping All Connected`
  (bind _result (`BlueprintSetLibrary.Set_ToArray` (`self.Connected Pawns`)))
  (for _array_element _result
    (`/Engine/EditorBlueprintResources/StandardMacros.IsValid` _array_element
      (:`Is Valid`
        (`/Game/Blueprints/AI_and_Enemies/AIPawn.Notify of Network Connection` _array_element self)))))

(fn `Remove Pawn from Network`
  (params (Pawn :type "/Game/Blueprints/AI_and_Enemies/AIPawn Object Reference"))
  (`BlueprintSetLibrary.Set_Remove` (`self.Connected Pawns`) Pawn))

(fn `UserConstructionScript`)