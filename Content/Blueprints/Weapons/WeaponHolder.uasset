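; WeaponHolder is a scene component that holds a list of weapon classes and manages the currently equipped weapon.
; NextWeapon and PrevWeapon cycle the index with wraparound, then Equip destroys the old weapon actor, spawns the selected class and snap-attaches it to the component.
; It equips on BeginPlay, records the weapon's display name, and forwards trigger and scope calls to the active weapon while tracking scoping state.
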(event `self.ReceiveBeginPlay`
  (`self.Equip`))

(fn `Equip`
  (bind _index (`self.Index`))
  (bind _weapon (`self.Weapon`))
  (bind _weapontypesheld (`self.WeaponTypesHeld`))
  (bind _output (`|GetArrayItem` _weapontypesheld _index))
  (if (`KismetArrayLibrary.Array_IsValidIndex` _weapontypesheld (`self.Index`))
    (`|ExecutionSequence`
      (:`then_0`
        ;[1 1 1] Unequip previous weapon
        (`/Engine/EditorBlueprintResources/StandardMacros.IsValid` _weapon
          (:`Is Valid`
            (`Actor.K2_DestroyActor` _weapon)
            (set `self.Weapon` null))))
      (:`then_1`
        (`KismetSystemLibrary.PrintString` (`KismetStringLibrary.Concat_StrStr` (`KismetStringLibrary.Conv_IntToString` _index) ": " (`KismetSystemLibrary.GetClassDisplayName` _output)))
        (bind _returnvalue (`|SpawnActorFromClass` _output (`self.K2_GetComponentToWorld`) "Undefined" "OverrideRootScale" null null))
        (bind _output_get (set `self.Weapon` _returnvalue))
        (`Actor.K2_AttachToComponent` _output_get self "None" "SnapToTarget" "SnapToTarget" "SnapToTarget" true)
        (set `self.WeaponName` (`KismetTextLibrary.Conv_StringToText` (`KismetSystemLibrary.GetDisplayName` _output_get)))))))

(fn `NextWeapon`
  (bind _returnvalue (+ (`self.Index`) 1))
  (set `self.Index` (select `bool` (>= _returnvalue (`KismetArrayLibrary.Array_Length` (`self.WeaponTypesHeld`))) :`false` _returnvalue))
  (`self.Equip`))

(fn `PrevWeapon`
  (bind _returnvalue (- (`self.Index`) 1))
  (set `self.Index` (select `bool` (< _returnvalue 0) :`false` _returnvalue :`true` (- (`KismetArrayLibrary.Array_Length` (`self.WeaponTypesHeld`)) 1)))
  (`self.Equip`))

(fn `ScopeEnd`
  (`/Game/Blueprints/Weapons/Weapons/Weapon.ScopeEnd` (`self.Weapon`))
  (set `self.isScoping` false))

(fn `ScopeStart`
  (`/Game/Blueprints/Weapons/Weapons/Weapon.ScopeBegin` (`self.Weapon`))
  (set `self.isScoping` true))

(fn `TriggerPull`
  (params (player :type "/Game/Blueprints/PlayerCharacter Object Reference"))
  (`/Game/Blueprints/Weapons/Weapons/Weapon.TriggerPull` (`self.Weapon`) player))

(fn `TriggerRelease`
  (`/Game/Blueprints/Weapons/Weapons/Weapon.TriggerRelease` (`self.Weapon`)))