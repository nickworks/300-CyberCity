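; AIPawn is an AI combatant with health, a friendly-or-hostile team flag and an alert state.
; AI Perception or Notify picks an opposing player or AIPawn as target, with Notify also waking sleeping pawns.
; Helper functions check sight by throttled raycast or perception, fire aimed projectiles on cooldown, explode, and time the return to Idle.
; ChangeState resets the timer and sets the state, including Dying at zero health, but its switch has no behavior attached.
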(event `self.ReceiveAnyDamage`
  (params (Damage :type "Float (single-precision)") (DamageType :type "DamageType Object Reference") (InstigatedBy :type "Controller Object Reference") (DamageCauser :type "Actor Object Reference"))
  ;[1 1 1] Take damage
  (bind _output_get (set `self.Health` (- (`self.Health`) Damage)))
  (if (<= _output_get 0.0)
    (`self.ChangeState` "NewEnumerator4")))

(event `self.AIPerception.OnPerceptionUpdated`
  (params (UpdatedActors :type "Array of Actor Object Reference (by ref)"))
  (if (`|EnumInequality` (`self.StateAlert`) "NewEnumerator8")
    (`self.CheckForPerception`)))

(fn `Awake`
  (if (`|EnumEquality` (`self.StateAlert`) "NewEnumerator8")
    (`self.ChangeState` "NewEnumerator0")))

(fn `ChangeState`
  (params (state :type "/Game/Blueprints/AIPawnStates Enum" :default "NewEnumerator0"))
  (`self.ResetChangeTimer`)
  (bind _output_get (set `self.StateAlert` state))
  (switch `/Game/Blueprints/AIPawnStates` _output_get))

(fn `CheckForPerception`
  (bind _outactors (`AIPerceptionComponent.GetCurrentlyPerceivedActors` (`self.AIPerception`) null))
  (if (not (<= (`KismetArrayLibrary.Array_Length` _outactors) 0))
    (for _array_element _outactors
      (if (not (`self.IsFriendly`))
        ;[1 1 1] Not friendly: scan for a player...
        (bind _asplayer_character (cast `/Game/Blueprints/PlayerCharacter` _array_element)
          (:`then`
            (set `self.SensedPawn` _asplayer_character)
            (set `self.SensedPawnLocation` (`self.K2_GetActorLocation` (`self.SensedPawn`)) :!label _label)
            (break))
          (:`CastFailed`
            ;[1 1 1] Friendly: scan for AIPawns
            (bind _asaipawn (cast `/Game/Blueprints/AIPawn` _array_element :!label _label_2))
            (if (!= (`/Game/Blueprints/AIPawn.IsFriendly` _asaipawn) (`self.IsFriendly`))
              (set `self.SensedPawn` _asaipawn)
              (goto _label))))
        (else
          (goto _label_2))))))

(fn `Explode`
  (`GameplayStatics.SpawnEmitterAtLocation` "/Game/Particles/Explosion.Explosion" (`self.K2_GetActorLocation`))
  (`self.K2_DestroyActor`))

(fn `InvestigateSensedPawn`
  (`/Engine/EditorBlueprintResources/StandardMacros.IsValid` (`self.SensedPawn`)
    (:`Is Valid`
      (`self.ChangeState` "NewEnumerator1"))))

(fn `IsAtTarget`
  (params (Threshold :type "Float (double-precision)" :default 200.0))
  (returns (IsAtTarget :type Boolean))
  (bind _threshold (`local.Threshold`))
  (return (<= (`KismetMathLibrary.VSizeSquared` (- (`self.SensedPawnLocation`) (`self.K2_GetActorLocation`))) (* _threshold _threshold))))

(fn `IsSensedPawnInSight`
  (params (CheckEvery :type "Float (double-precision)" :default 0.5) (DoARaycast :type Boolean))
  (returns (IsPawnSeen :type Boolean) (LookedThisFrame :type Boolean))
  ;[1 1 1] Cooldown
  (if (> (`self.CooldownScan`) 0.0)
    (set `self.CooldownScan` (- (`self.CooldownScan`) (`GameplayStatics.GetWorldDeltaSeconds`)))
    (return false false)
    (else
      (set `self.CooldownScan` CheckEvery)
      (`/Engine/EditorBlueprintResources/StandardMacros.IsValid` (`self.SensedPawn`)
        (:`Is Valid`
          (if DoARaycast
            ;[1 1 1] Raycasting
            (bind (_outhit _returnvalue) (`KismetSystemLibrary.LineTraceSingle` :`Start` (`self.K2_GetActorLocation`) :`End` (`self.K2_GetActorLocation` (`self.SensedPawn`)) :`TraceChannel` "TraceTypeQuery1" :`DrawDebugType` "ForDuration" :`DrawTime` 0.5))
            (if (and (not _returnvalue) (<= (`.Distance` (`GameplayStatics.BreakHitResult` _outhit)) (`self.MaxVisibilityDistance`)))
              (set `self.SensedPawnLocation` (`self.K2_GetActorLocation` (`self.SensedPawn`)))
              (return true true))
            (else
              ;[1 1 1] Check AIPerception whether or not the pawn is SEEN
              (if (>= (`KismetArrayLibrary.Array_Find` (`AIPerceptionComponent.GetCurrentlyPerceivedActors` (`self.AIPerception`) "/Script/AIModule.AISense_Sight") (`self.SensedPawn`)) 0)
                (set `self.SensedPawnLocation` (`self.K2_GetActorLocation` (`self.SensedPawn`)))
                (return true true)
                (else
                  (return false true))))))
        (:`Is Not Valid`
          (return false true))))))

(fn `Notify`
  (params (TriggeringPawn :type "Pawn Object Reference"))
  (bind _sensedpawn (`self.SensedPawn`))
  (bind _triggeringpawn (`local.TriggeringPawn`))
  (`self.Awake`)
  (bind _asaipawn (cast `/Game/Blueprints/AIPawn` TriggeringPawn)
    (:`then`
      ;[1 1 1] Trigger is an AI
      (if (!= (`/Game/Blueprints/AIPawn.IsFriendly` _asaipawn) (`self.IsFriendly`))
        (`/Engine/EditorBlueprintResources/StandardMacros.IsValid` _sensedpawn :!label _label ; If I don't already have a target...
          (:`Is Valid`
            (`KismetSystemLibrary.PrintString` (`KismetStringLibrary.Concat_StrStr` "No thanks, I'm already targeting a " (`KismetSystemLibrary.GetDisplayName` _sensedpawn))))
          (:`Is Not Valid`
            ;[1 1 1] Set this as a new target for me
            (set `self.SensedPawn` _triggeringpawn)
            (set `self.SensedPawnLocation` (`self.K2_GetActorLocation` _triggeringpawn))))))
    (:`CastFailed`
      ;[1 1 1] Trigger is a Player
      (if (`self.IsFriendly`)
        (`KismetSystemLibrary.PrintString` "I'm too friendly to attack the player")
        (else
          (goto _label))))))

(fn `ResetChangeTimer`
  (set `self.StateChangeTimer` 0.0))

(fn `ShootAtPlayer`
  (params (`Projectile Type` :type "/Game/Blueprints/Weapons/Projectiles/Projectile Class Reference") (ShootOrigin :type "Vector Structure") (ShootCooldown :type "Float (double-precision)" :default 0.5))
  ;[1 1 1] Cooldown
  (if (>= (`self.CooldownShoot`) 0.0)
    (set `self.CooldownShoot` (- (`self.CooldownShoot`) (`GameplayStatics.GetWorldDeltaSeconds`)))
    (else
      (set `self.CooldownShoot` ShootCooldown)
      (`/Engine/EditorBlueprintResources/StandardMacros.IsValid` (`self.SensedPawn`)
        (:`Is Valid`
          (`|SpawnActorFromClass` (`local.Projectile Type`) (`KismetMathLibrary.MakeTransform` (`local.ShootOrigin`) (`KismetMathLibrary.FindLookAtRotation` (`local.ShootOrigin`) (`self.K2_GetActorLocation` (`self.SensedPawn`)))) "Undefined" "OverrideRootScale" null null))))))

(fn `UserConstructionScript`)

(fn `WaitThenGoIdle`
  (params (Delay :type "Float (double-precision)"))
  (bind _output_get (set `self.StateChangeTimer` (+ (`self.StateChangeTimer`) (`GameplayStatics.GetWorldDeltaSeconds`))))
  (if (>= _output_get Delay)
    (set `self.SensedPawn` null)
    (`self.ChangeState` "NewEnumerator0")))