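; In-world upgrade terminal where the player changes installed MODs, doubling as a checkpoint that sets the GameMode spawn transform on use.
; A trigger box enables Interact, which brightens the screen material and spotlight and scales up a WidgetTerminal via timeline, reversed on exit.
; Widget changes are written to CyborgPlayer's MODsInstalled and refreshed in the GUI.
; While open, Tick eases the widget's pitch against the player's view pitch.
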(event `InputAction|Interact` :consume false
  (params (Key :type "Key Structure"))
  (:`Pressed`
    (if (not (`self.is Showing Screen`))
      (set `self.is Showing Screen` true)
      (`self.Set Spawn Point Here`)
      (`MaterialInstanceDynamic.SetScalarParameterValue` (`self.ScreenMaterial`) "GlowIntensity" 10.0)
      (`LightComponent.SetIntensity` (`self.SpotLight`) 3000.0)
      (`self.UpdateTheGUI`)
      (`SceneComponent.SetVisibility` (`self.Widget`) true false)
      (`/Game/Blueprints/Widgets/WidgetTerminal.Anim - Load MODS` (`self.GUI Reference`))
      (`SceneComponent.SetVisibility` (`self.Widget`) true false)
      (bind (_direction _scale_of_screen) (`Timeline|Display Widget` :!label _label)
        (:`Update`
          (`SceneComponent.SetRelativeScale3D` (`self.Widget`) (`KismetMathLibrary.Conv_DoubleToVector` (* _scale_of_screen 0.08))))
        (:`Finished`
          (switch `ETimelineDirection` _direction
            (:`Forward`
              (`SceneComponent.SetVisibility` (`self.Widget`) true false))
            (:`Backward`
              (`SceneComponent.SetVisibility` (`self.Widget`) false false))))))))

(event `self.Box.OnComponentBeginOverlap`
  (params (OverlappedComponent :type "PrimitiveComponent Object Reference") (OtherActor :type "Actor Object Reference") (OtherComp :type "PrimitiveComponent Object Reference") (OtherBodyIndex :type Integer) (bFromSweep :type Boolean) (SweepResult :type "HitResult Structure (by ref)"))
  (`self.EnableInput` (`GameplayStatics.GetPlayerController` 0)))

(event `self.Box.OnComponentEndOverlap`
  (params (OverlappedComponent :type "PrimitiveComponent Object Reference") (OtherActor :type "Actor Object Reference") (OtherComp :type "PrimitiveComponent Object Reference") (OtherBodyIndex :type Integer))
  (`self.DisableInput` (`GameplayStatics.GetPlayerController` 0))
  (set `self.is Showing Screen` false)
  (`MaterialInstanceDynamic.SetScalarParameterValue` (`self.ScreenMaterial`) "GlowIntensity" 1.0 :!label _label_2)
  (`LightComponent.SetIntensity` (`self.SpotLight`) 1000.0)
  (`/Game/Blueprints/Widgets/WidgetTerminal.Anim - Fade Away` (`self.GUI Reference`))
  (goto _label :!via `Reverse`))

(event `self.ReceiveBeginPlay`
  (bind _aswidget_terminal (cast `/Game/Blueprints/Widgets/WidgetTerminal` (`WidgetComponent.GetUserWidgetObject` (`self.Widget`))))
  (bind _output_get (set `self.GUI Reference` _aswidget_terminal))
  (add `/Game/Blueprints/Widgets/WidgetTerminal.Close It` _output_get (delegate `CLOSE`))
  (add `/Game/Blueprints/Widgets/WidgetTerminal.StateChanged` (`self.GUI Reference`) (delegate `STATE CHANGED`))
  ;[1 1 1] Setup dynamic material for glowing computer screen
  (bind _returnvalue (`PrimitiveComponent.CreateDynamicMaterialInstance` (`self.Screen`) 0 "/Game/ArtKits/Materials/GlowTerminalMonitor.GlowTerminalMonitor" "None"))
  (set `self.ScreenMaterial` _returnvalue)
  (goto _label_2))

(event `STATE CHANGED`
  (params (`New Ability Set` :type "/Game/Blueprints/PlayerStuff/PlayerAbilitySet Structure"))
  (bind _ascyborg_player (cast `/Game/Blueprints/PlayerStuff/CyborgPlayer` (`GameplayStatics.GetPlayerCharacter` 0)))
  (bind _output_get (set `/Game/Blueprints/PlayerStuff/CyborgPlayer.MODs Installed` `New Ability Set` _ascyborg_player))
  (`/Game/Blueprints/Widgets/WidgetTerminal.Update State` (`self.GUI Reference`) _output_get (`/Game/Blueprints/PlayerStuff/CyborgPlayer.GB TOTAL` _ascyborg_player)))

(event `CLOSE`)

(event `self.ReceiveTick`
  (params (DeltaSeconds :type "Float (single-precision)"))
  (if (`self.is Showing Screen`)
    (`SceneComponent.K2_SetRelativeRotation` (`self.Widget`) (`KismetMathLibrary.RInterpTo` (`SceneComponent.RelativeRotation` (`self.Widget`)) (`KismetMathLibrary.MakeRotator` 0.0 (* (.pitch (`.OutRotation` (`self.GetActorEyesViewPoint` (`GameplayStatics.GetPlayerController` 0)))) -1.0) 90.0) DeltaSeconds 4.0) false false)))

(fn `Set Spawn Point Here`
  (bind _asgame_mode_cyborg_player (cast `/Game/Blueprints/PlayerStuff/GameMode_CyborgPlayer` (`GameplayStatics.GetGameMode`)))
  (set `/Game/Blueprints/PlayerStuff/GameMode_CyborgPlayer.SpawnTransform` (`self.GetTransform` (`GameplayStatics.GetPlayerCharacter` 0)) _asgame_mode_cyborg_player)
  (`KismetSystemLibrary.PrintString` "Spawn point set"))

(fn `UpdateTheGUI`
  (bind _ascyborg_player (cast `/Game/Blueprints/PlayerStuff/CyborgPlayer` (`GameplayStatics.GetPlayerCharacter` 0)))
  (`/Game/Blueprints/Widgets/WidgetTerminal.Update State` (`self.GUI Reference`) (`/Game/Blueprints/PlayerStuff/CyborgPlayer.MODs Installed` _ascyborg_player) (`/Game/Blueprints/PlayerStuff/CyborgPlayer.GB TOTAL` _ascyborg_player)))

(fn `UserConstructionScript`)