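; A heat-seeking projectile actor that homes in on the first player character and explodes when damaged.
; Every tick it accelerates its capsule toward a clamped desired velocity based on the offset to the target, minus current velocity, and rotates to face its movement.
; Taking any damage disables further damage, applies radial damage, spawns an explosion emitter and destroys the actor.
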(event `self.ReceiveBeginPlay`
  (set `self.target` (`GameplayStatics.GetPlayerCharacter` 0)))

(event `self.ReceiveTick`
  (params (DeltaSeconds :type "Float (single-precision)"))
  (`self.SteerTowardsTarget`))

(event `self.ReceiveAnyDamage`
  (params (Damage :type "Float (single-precision)") (DamageType :type "DamageType Object Reference") (InstigatedBy :type "Controller Object Reference") (DamageCauser :type "Actor Object Reference"))
  (`KismetSystemLibrary.PrintString` "ouch")
  (`self.Explode`))

(fn `Explode`
  (bind _returnvalue (`self.K2_GetActorLocation`))
  (set `self.bCanBeDamaged` false)
  (`GameplayStatics.ApplyRadialDamage` :`BaseDamage` 50.0 :`Origin` _returnvalue :`DamageRadius` 200.0 :`DamageCauser` null :`InstigatedByController` null)
  (`GameplayStatics.SpawnEmitterAtLocation` "/Game/Particles/Explosion.Explosion" _returnvalue)
  (`self.K2_DestroyActor`))

(fn `SteerTowardsTarget`
  (bind _returnvalue (`self.GetVelocity`))
  (bind _returnvalue_2 (`self.K2_GetActorLocation`))
  (`/Engine/EditorBlueprintResources/StandardMacros.IsValid` (`self.target`)
    (:`Is Valid`
      (`PrimitiveComponent.AddForce` (`self.Capsule`) (- (`KismetMathLibrary.ClampVectorSize` (* (- (`self.K2_GetActorLocation` (`self.Target`)) (`self.K2_GetActorLocation`)) (`self.thrustAmount`)) 0.0 (`self.MAX_SPEED`)) _returnvalue) "None" true)
      (`self.K2_SetActorRotation` (`KismetMathLibrary.FindLookAtRotation` _returnvalue_2 (+ _returnvalue_2 _returnvalue))))))

(fn `UserConstructionScript`
  (`ParticleSystemComponent.SetFloatParameter` (`self.ParticleSystem`) "Rate" 1.0))