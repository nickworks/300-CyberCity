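; Environment kit path tool that lays a chosen static mesh along an editable spline as instanced pieces.
; The construction script splits each segment between spline points into a set number of equal steps, placing an instance at each step's midpoint.
; Each instance follows the spline's rotation, scales its length to the step with adjustable width and height, and gets a random vertical offset.
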(fn `UserConstructionScript`
  (locals (`temp dis incr` :type "Float (double-precision)" :default 0.0) (`temp dis` :type "Float (double-precision)" :default 0.0))
  (bind _temp_dis (`local.temp dis`))
  (bind _rand_z (`self.Rand Z`))
  (bind _spline (`self.Spline`))
  (bind _spline_2 (`self.Spline`))
  (bind _returnvalue (- (`SplineComponent.GetNumberOfSplinePoints` (`self.Spline`)) 1))
  (`StaticMeshComponent.SetStaticMesh` (`self.InstancedStaticMesh`) (`self.Mesh to Use`))
  (for _index (range (+ _returnvalue 1))
    (if (< _index _returnvalue)
      (bind _returnvalue_2 (`SplineComponent.GetDistanceAlongSplineAtSplinePoint` _spline _index))
      (bind _output_get (set `local.temp dis` _returnvalue_2))
      (bind _output_get_2 (set `local.temp dis incr` (/ (- (`SplineComponent.GetDistanceAlongSplineAtSplinePoint` _spline (+ _index 1)) _returnvalue_2) (`KismetMathLibrary.Conv_IntToDouble` (`self.iterations`)))))
      (set `local.temp dis` (+ _output_get (/ _output_get_2 2.0)))
      (for _ (range 1 (+ (`self.iterations`) 1))
        (`InstancedStaticMeshComponent.AddInstance` (`self.InstancedStaticMesh`) (`KismetMathLibrary.MakeTransform` (+ (`SplineComponent.GetLocationAtDistanceAlongSpline` _spline_2 _temp_dis "Local") (`KismetMathLibrary.MakeVector` 0.0 0.0 (`KismetMathLibrary.RandomFloatInRange` (* _rand_z -1.0) _rand_z))) (`SplineComponent.GetRotationAtDistanceAlongSpline` _spline_2 _temp_dis "Local") (`KismetMathLibrary.MakeVector` (* (`local.temp dis incr`) (`self.Scale Length`) 0.01) (`self.Scale Width`) (`self.Scale Height`))))
        (set `local.temp dis` (+ (`local.temp dis`) (`local.temp dis incr`)))))))