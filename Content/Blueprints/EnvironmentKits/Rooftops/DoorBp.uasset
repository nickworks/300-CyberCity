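; DoorBp is an interactable hinged door for the Rooftops environment kit that swings away from the player when opened.
; A collider overlap with CyborgPlayer enables input on the door, so the Interact action toggles it open or closed.
; The dot product of the player's offset and the hinge's forward vector picks the swing direction.
; The OpenDoor timeline drives the hinge yaw, reverses to close, and sets IsOpen when finished.
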(event `Open the Door`
  (params (Pawn :type "Pawn Object Reference"))
  (bind (_returnvalue_x _returnvalue_y) (`KismetMathLibrary.BreakVector` (- (`self.K2_GetActorLocation` Pawn) (`self.K2_GetActorLocation`))))
  (set `self.direction` (select `bool` (> (`KismetMathLibrary.Dot_VectorVector` (`KismetMathLibrary.Normal` (`KismetMathLibrary.MakeVector` _returnvalue_x _returnvalue_y)) (`SceneComponent.GetForwardVector` (`self.HINGE`))) 0.0) :`false` 1 :`true` -1))
  (bind (_direction _percent) (`Timeline|OpenDoor` :!label _label)
    (:`Update`
      (`SceneComponent.K2_SetRelativeRotation` (`self.HINGE`) (`KismetMathLibrary.MakeRotator` 0.0 0.0 (* _percent (`KismetMathLibrary.Conv_IntToDouble` (`self.direction`)) 80.0)) false false))
    (:`Finished`
      (switch `ETimelineDirection` _direction
        (:`Forward`
          (set `self.isOpen` true))
        (:`Backward`
          (set `self.isOpen` false))))))

(event `Close the Door`
  (goto _label :!via `Reverse`))

(event `self.Collider.OnComponentBeginOverlap`
  (params (OverlappedComponent :type "PrimitiveComponent Object Reference") (OtherActor :type "Actor Object Reference") (OtherComp :type "PrimitiveComponent Object Reference") (OtherBodyIndex :type Integer) (bFromSweep :type Boolean) (SweepResult :type "HitResult Structure (by ref)"))
  (cast `/Game/Blueprints/PlayerStuff/CyborgPlayer` OtherActor)
  (`self.EnableInput` (`GameplayStatics.GetPlayerController` 0)))

(event `self.Collider.OnComponentEndOverlap`
  (params (OverlappedComponent :type "PrimitiveComponent Object Reference") (OtherActor :type "Actor Object Reference") (OtherComp :type "PrimitiveComponent Object Reference") (OtherBodyIndex :type Integer))
  (cast `/Game/Blueprints/PlayerStuff/CyborgPlayer` OtherActor)
  (`self.DisableInput` (`GameplayStatics.GetPlayerController` 0)))

(event `InputAction|Interact` :consume false
  (params (Key :type "Key Structure"))
  (:`Pressed`
    (if (`self.isOpen`)
      (`self.Close the Door`)
      (else
        (`self.Open the Door` (`GameplayStatics.GetPlayerPawn` 0))))))

(fn `UserConstructionScript`)