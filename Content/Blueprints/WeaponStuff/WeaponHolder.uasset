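; Weapon holder scene component that manages the weapon carried by its CyborgPlayer owner.
; Cycles an index through the held weapon classes with wraparound, blocking switches while scoping, and equips the starting weapon on BeginPlay.
; Equipping caches the old weapon's ammo and destroys it, then spawns the new one attached to the component and passes it the player.
; Scope, trigger and reload calls are forwarded to the current weapon.
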(event `self.ReceiveBeginPlay`
  (`self.Equip`))

(fn `Dispose`
  (bind _weapon (`self.Weapon`))
  (`/Engine/EditorBlueprintResources/StandardMacros.IsValid` _weapon
    (:`Is Valid`
      (`Actor.K2_DestroyActor` _weapon))))

(fn `Equip`
  (locals (ClassOfSpawnedWeapon :type "/Game/Blueprints/WeaponStuff/BaseWeapon Class Reference"))
  (bind _weapon (`self.Weapon`))
  (bind _weapontypesheld (`self.WeaponTypesHeld`))
  (if (`KismetArrayLibrary.Array_IsValidIndex` _weapontypesheld (`self.Index`))
    (`|ExecutionSequence`
      (:`then_0`
        ;[1 1 1] Unequip previous weapon
        (`/Engine/EditorBlueprintResources/StandardMacros.IsValid` _weapon
          (:`Is Valid`
            (`/Game/Blueprints/WeaponStuff/BaseWeapon.CacheAmmo` _weapon)
            (`Actor.K2_DestroyActor` _weapon)
            (set `self.Weapon` null))))
      (:`then_1`
        (set `local.ClassOfSpawnedWeapon` (`|GetArrayItem` _weapontypesheld (`self.Index`)))
        (bind _returnvalue (`|SpawnActorFromClass` (`local.ClassOfSpawnedWeapon`) (`self.K2_GetComponentToWorld`) "Undefined" "OverrideRootScale" null null))
        (bind _output_get (set `self.Weapon` _returnvalue))
        (`Actor.K2_AttachToComponent` _output_get self "None" "SnapToTarget" "SnapToTarget" "SnapToTarget" true)
        (bind _ascyborg_player (cast `/Game/Blueprints/PlayerStuff/CyborgPlayer` (`self.GetOwner`)))
        (`/Game/Blueprints/WeaponStuff/BaseWeapon.SetPlayerCharacter` (`self.Weapon`) _ascyborg_player)))))

(fn `NextWeapon`
  (bind _returnvalue (+ (`self.Index`) 1))
  (if (not (`self.isScoping`))
    (set `self.Index` (select `bool` (>= _returnvalue (`KismetArrayLibrary.Array_Length` (`self.WeaponTypesHeld`))) :`false` _returnvalue))
    (`self.Equip`)))

(fn `PrevWeapon`
  (bind _returnvalue (- (`self.Index`) 1))
  (if (not (`self.isScoping`))
    (set `self.Index` (select `bool` (< _returnvalue 0) :`false` _returnvalue :`true` (- (`KismetArrayLibrary.Array_Length` (`self.WeaponTypesHeld`)) 1)))
    (`self.Equip`)))

(fn `Reload`
  (`/Game/Blueprints/WeaponStuff/BaseWeapon.Reload` (`self.Weapon`)))

(fn `ScopeEnd`
  (bind _weapon (`self.Weapon`))
  (`/Game/Blueprints/WeaponStuff/BaseWeapon.ScopeEnd` _weapon)
  (bind _output_get (set `self.isScoping` false))
  (set `/Game/Blueprints/WeaponStuff/BaseWeapon.isScoping` _output_get _weapon))

(fn `ScopeStart`
  (bind _weapon (`self.Weapon`))
  (`/Game/Blueprints/WeaponStuff/BaseWeapon.ScopeBegin` _weapon)
  (bind _output_get (set `self.isScoping` true))
  (set `/Game/Blueprints/WeaponStuff/BaseWeapon.isScoping` _output_get _weapon))

(fn `TriggerPull`
  (`/Game/Blueprints/WeaponStuff/BaseWeapon.TriggerPull` (`self.Weapon`)))

(fn `TriggerRelease`
  (`/Game/Blueprints/WeaponStuff/BaseWeapon.TriggerRelease` (`self.Weapon`)))