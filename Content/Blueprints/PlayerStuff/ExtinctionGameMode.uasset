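; ExtinctionGameMode handles player respawning and holds the player's ammo state.
; Respawn spawns a new PlayerCharacter and has player controller 0 possess it.
; AmmoPools map stores reserves by type: UsePoolAmmo moves rounds into a by-ref clip up to capacity, and PickupAmmo adds without clamping to Max.
; A separate AmmoInGuns map caches loaded ammo per gun type, with lookups reporting whether an entry exists.
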(fn `CacheGunAmmo`
  (params (GunType :type "/Game/Blueprints/Weapons/Weapons/BaseWeapon Soft Class Reference") (Amount :type Integer))
  (`BlueprintMapLibrary.Map_Add` (`self.AmmoInGuns`) GunType Amount))

(fn `GetAmmoInGun`
  (params (`Gun Type` :type "/Game/Blueprints/Weapons/Weapons/BaseWeapon Soft Class Reference"))
  (returns (Ammo :type Integer) (CacheExists :type Boolean))
  (bind (_value _returnvalue) (`BlueprintMapLibrary.Map_Find` (`self.AmmoInGuns`) `Gun Type`))
  (return (select `bool` _returnvalue :`true` _value) _returnvalue))

(fn `PickupAmmo`
  (params (Type :type "/Game/Blueprints/Weapons/AmmoType Enum" :default "NewEnumerator0") (Amount :type "Float (double-precision)"))
  (bind _ammopools (`self.AmmoPools`))
  (bind _value (`BlueprintMapLibrary.Map_Find` _ammopools Type))
  (`BlueprintMapLibrary.Map_Add` _ammopools Type (make `/Game/Blueprints/Weapons/AmmoPool` (+ (break `/Game/Blueprints/Weapons/AmmoPool` _value) Amount) (`.Max_5_DAF73E1D4289EE23EC01B7A8042C00C2` (break `/Game/Blueprints/Weapons/AmmoPool` _value)) (`.Type_8_7EE0E82E442640A975312ABFE9A57420` (break `/Game/Blueprints/Weapons/AmmoPool` _value)))))

(fn `Respawn`
  (bind _returnvalue (`|SpawnActorFromClass` "/Game/Blueprints/PlayerStuff/PlayerCharacter.PlayerCharacter_C" (`self.SpawnTransform`) "Undefined" "OverrideRootScale" null null))
  (`Controller.Possess` (`GameplayStatics.GetPlayerController` 0) _returnvalue))

(fn `UsePoolAmmo`
  (params (Clip :type "/Game/Blueprints/Weapons/AmmoPool Structure (by ref)"))
  (locals (ReloadAmount :type "Float (double-precision)"))
  (bind (_current _max _type) (break `/Game/Blueprints/Weapons/AmmoPool` Clip))
  (bind (_current_2 _max_2 _type_2) (break `/Game/Blueprints/Weapons/AmmoPool` Clip))
  (bind (_current_3 _max_3 _type_3) (break `/Game/Blueprints/Weapons/AmmoPool` (`BlueprintMapLibrary.Map_Find` (`self.AmmoPools`) _type)))
  (bind _output_get (set `local.ReloadAmount` (`KismetMathLibrary.FMin` _current_3 (- _max _current))))
  (`|VariableSetRef` Clip (make `/Game/Blueprints/Weapons/AmmoPool` (+ _current_2 _output_get) _max_2 _type_2))
  (bind _ammopool (make `/Game/Blueprints/Weapons/AmmoPool` (- _current_3 _output_get) _max_3 _type_3))
  (`BlueprintMapLibrary.Map_Add` (`self.AmmoPools`) (`.Type_8_7EE0E82E442640A975312ABFE9A57420` (break `/Game/Blueprints/Weapons/AmmoPool` _ammopool)) _ammopool))

(fn `UserConstructionScript`)