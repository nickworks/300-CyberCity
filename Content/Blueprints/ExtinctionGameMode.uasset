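; Game mode for Extinction that handles player respawning and stores the player's ammo state.
; Respawn spawns a new PlayerCharacter at the stored SpawnTransform and has player controller 0 possess it.
; UsePoolAmmo draws from per-type ammo pools, capping each request at what remains.
; A separate per-gun map caches loaded ammo, with lookups reporting whether a cached value exists.
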(fn `CacheGunAmmo`
  (params (GunType :type "/Game/Blueprints/Weapons/Weapons/BaseWeapon Soft Class Reference") (Amount :type Integer))
  (`BlueprintMapLibrary.Map_Add` (`self.AmmoInGuns`) GunType Amount))

(fn `GetAmmoInGun`
  (params (`Gun Type` :type "/Game/Blueprints/Weapons/Weapons/BaseWeapon Soft Class Reference"))
  (returns (Ammo :type Integer) (CacheExists :type Boolean))
  (bind (_value _returnvalue) (`BlueprintMapLibrary.Map_Find` (`self.AmmoInGuns`) `Gun Type`))
  (return (select `bool` _returnvalue :`true` _value) _returnvalue))

(fn `Respawn`
  (bind _returnvalue (`|SpawnActorFromClass` "/Game/Blueprints/PlayerCharacter.PlayerCharacter_C" (`self.SpawnTransform`) "Undefined" "OverrideRootScale" null null))
  (`Controller.Possess` (`GameplayStatics.GetPlayerController` 0) _returnvalue))

(fn `UsePoolAmmo`
  (params (`Ammo Type` :type "/Game/Blueprints/Weapons/AmmoType Enum" :default "NewEnumerator0") (`Amount Requested` :type Integer))
  (returns (AmmoAvailable :type Integer))
  (bind (_value _returnvalue) (`BlueprintMapLibrary.Map_Find` (`self.AmmoPools`) `Ammo Type`))
  (bind _returnvalue_2 (`KismetMathLibrary.Min` _value `Amount Requested`))
  (if _returnvalue
    (`BlueprintMapLibrary.Map_Add` (`self.AmmoPools`) `Ammo Type` (- _value _returnvalue_2))
    (return _returnvalue_2)
    (else
      (return 0))))

(fn `UserConstructionScript`)